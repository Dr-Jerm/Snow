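; Base VR pawn that replicates the player's head and hand poses for multiplayer.
; Every Tick, the locally controlled instance reads HMD and motion controller transforms and sends them through Server events.
; These relay to Broadcast events, which set the relative transforms of the replicated head and two hand meshes directly, without smoothing.
; Left and right trigger presses only print debug text.
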(event EventBeginPlay)

(event EventActorBeginOverlap
  (params (OtherActor :type Actor%20Object%20Reference)))

(event EventTick
  (params (DeltaSeconds :type Float%20%28single-precision%29))
  (CallFunction|ProccessHead)
  (CallFunction|ProcessHands))

(event Input|KeyboardEvents|MotionControllerRightTrigger
  (params (Key :type Key%20Structure :default "AnyKey"))
  (:Pressed
    (Development|PrintText "RightTriggerPressed")))

(event Input|KeyboardEvents|MotionControllerLeftTrigger
  (params (Key :type Key%20Structure :default "AnyKey"))
  (:Pressed
    (Development|PrintText "LeftTriggerPressed")))

(event Custom|BroadcastHeadUpdate
  (params (Rotation :type Rotator) (Position :type Vector))
  (Transformation|SetRelativeLocationAndRotation (Variables|Default|GetReplicatedHead) Position Rotation false false))

(event Custom|ServerUpdateHead
  (params (Rotation :type Rotator) (Position :type Vector))
  (CallFunction|BroadcastHeadUpdate Rotation Position))

(event Custom|ServerUpdateHands
  (params (LeftHandPosition :type Vector) (LeftHandRotation :type Rotator) (RightHandPosition :type Vector) (RightHandRotation :type Rotator))
  (CallFunction|BroadcastHandUpdate LeftHandPosition LeftHandRotation RightHandPosition RightHandRotation))

(event Custom|BroadcastHandUpdate
  (params (LeftHandPosition :type Vector) (LeftHandRotaton :type Rotator) (RightHandPosition :type Vector) (RightHandRotation :type Rotator))
  (Utilities|FlowControl|Sequence
    (:then_0
      (Transformation|SetRelativeLocationAndRotation (Variables|Default|GetReplicatedLeftHandMesh) LeftHandPosition LeftHandRotaton false false))
    (:then_1
      (Transformation|SetRelativeLocationAndRotation (Variables|Default|GetReplicatedRightHandMesh) RightHandPosition RightHandRotation false false))))

(fn ConstructionScript)

(fn ProccessHead
  (bind (_devicerotation _deviceposition) (Class|HeadMountedDisplayFunctionLibrary|GetOrientationandPosition))
  (if (Pawn|IsLocallyControlled)
    (CallFunction|ServerUpdateHead _devicerotation _deviceposition))
  (return))

(fn ProcessHands
  (bind (_outposition _outorientation) (Class|SteamVRFunctionLibrary|GetHandPositionandOrientation 0 "Right"))
  (bind (_outposition_2 _outorientation_2) (Class|SteamVRFunctionLibrary|GetHandPositionandOrientation 0 "Left"))
  (if (Pawn|IsLocallyControlled)
    (CallFunction|ServerUpdateHands _outposition_2 _outorientation_2 _outposition _outorientation)))