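; Game mode for a multiplayer VR brawl that handles player joining and timed match flow.
; On login, the server spawns and possesses a VR pawn at round-robin PlayerStarts, randomizes its customization, and registers a score slot through the snow game and player states.
; Server world time drives match start and end, then Tick server-travels to the "rag" map after the end wait.
; A broadcast event also exposes RestartGame.
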(event EventPostLogin
  (params (NewPlayer :type Player%20Controller%20Object%20Reference))
  (Networking|SwitchHasAuthority
    (:Authority
      (bind _asbase_player_controller_bp (Utilities|Casting|CastToBasePlayerControllerBP NewPlayer))
      (bind _outactors (Actor|GetAllActorsOfClass "/Script/Engine.PlayerStart"))
      (bind _returnvalue (Game|SpawnActorfromClass "/Game/VRPlayer/VRBaseBP.VRBaseBP_C" (Math|Conversions|ToTransform(Vector) (Transformation|GetActorLocation (Utilities|Array|Get(acopy) _outactors (Math|Integer|%(Integer) (Variables|Default|GetSpawnOrder) (Utilities|Array|Length _outactors))))) "AlwaysSpawn" 0 0))
      (Pawn|Possess _asbase_player_controller_bp _returnvalue)
      (Default|ClientPostLogin _asbase_player_controller_bp)
      (Variables|/Script/Snow.VRBase|SetCustomization _returnvalue (Utilities|Array|MakeArray (Math|Integer|%(Integer) (Math|Random|RandomInteger 10) 2) (Math|Integer|%(Integer) (Math|Random|RandomInteger 10) 2) (Math|Integer|%(Integer) (Math|Random|RandomInteger 10) 2) (Math|Integer|%(Integer) (Math|Random|RandomInteger 10) 2) (Math|Integer|%(Integer) (Math|Random|RandomInteger 10) 2)))
      (Default|VisualChange _returnvalue)
      (bind _assnow_game_state_bp (Utilities|Casting|CastToSnowGameStateBP (Game|GetGameState)))
      (bind _assnow_player_state_bp (Utilities|Casting|CastToSnowPlayerStateBP (Variables|/Script/Engine.Controller|GetPlayerState _asbase_player_controller_bp)))
      (bind _playerscoreindex (Class|SnowGameState|PlayerJoin _assnow_game_state_bp (Variables|/Script/Engine.PlayerState|GetPlayerId _assnow_player_state_bp)))
      (Variables|/Script/Snow.SnowPlayerState|SetScoreIndex _assnow_player_state_bp _playerscoreindex)
      (Variables|Default|SetSpawnOrder (+ (Variables|Default|GetSpawnOrder) 1))
      (Variables|/Game/VRPlayer/SnowPlayerStateBP.SnowPlayerStateBP_C|SetpawnReference _assnow_player_state_bp _returnvalue))))

(event EventTick
  (params (DeltaSeconds :type Float%20%28single-precision%29))
  (Networking|SwitchHasAuthority
    (:Authority
      (if (> (GameState|GetServerWorldTimeSeconds (Game|GetGameState)) (+ (Variables|Default|GetStartWaitLength) (Variables|Default|GetGameLength) (Variables|Default|GetEndWaitLength)))
        (Development|ExecuteConsoleCommand "ServerTravel rag?listen")))))

(event EventOnSetMatchState
  (params (NewState :type Name)))

(event Custom|BroadcastRestart
  (Class|GameMode|RestartGame))

(event Custom|ServerRestart
  (CallFunction|BroadcastRestart))

(fn ConstructionScript)

(fn ReadytoStartMatch
  (return (> (GameState|GetServerWorldTimeSeconds (Game|GetGameState)) (Variables|Default|GetStartWaitLength))))

(fn ReadytoEndMatch
  (return (> (GameState|GetServerWorldTimeSeconds (Game|GetGameState)) (+ (Variables|Default|GetStartWaitLength) (Variables|Default|GetGameLength)))))