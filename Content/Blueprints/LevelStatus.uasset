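; LevelStatus is an actor that shows the match status on a TextRender in the snow game.
; Every Tick it switches on the game state's MatchState, showing a start prompt, blank text, or the result.
; After the match it sums GetScore for each player against all players in PlayerArray, then announces the top player's ID or a tie.
; CurrentScore is never reset between players or ticks, so totals accumulate.
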(event EventBeginPlay)

(event Collision|EventActorBeginOverlap
  (params (OtherActor :type Actor%20Object%20Reference)))

(event EventTick
  (params (DeltaSeconds :type Float%20%28single-precision%29))
  (switch name (Variables|/Script/Engine.GameState|GetMatchState (Game|GetGameState))
    (:WaitingToStart
      (Variables|Default|SetMatchText "Get Ready to Begin!"))
    (:InProgress
      (Variables|Default|SetMatchText ""))
    (:WaitingPostMatch
      (bind _assnow_game_state_bp (Utilities|Casting|CastToSnowGameStateBP (Game|GetGameState)))
      (Variables|Default|SetSnowGameState _assnow_game_state_bp)
      (bind _assnow_player_state_bp (Utilities|Casting|CastToSnowPlayerStateBP (Utilities|Array|Get(acopy) (Variables|/Script/Engine.GameState|GetPlayerArray _assnow_game_state_bp))))
      (Variables|Default|SetHighestPlayers (Utilities|Array|MakeArray _assnow_player_state_bp))
      (Variables|Default|SetHighestScores (Utilities|Array|MakeArray -99999999))
      (for _array_element (Variables|/Script/Engine.GameState|GetPlayerArray _assnow_game_state_bp)
        (bind _assnow_player_state_bp_2 (Utilities|Casting|CastToSnowPlayerStateBP _array_element))
        (Variables|Default|SetCurrentPlayer _assnow_player_state_bp_2)
        (for _array_element_2 (Variables|/Script/Engine.GameState|GetPlayerArray _assnow_game_state_bp)
          (bind _assnow_player_state_bp_3 (Utilities|Casting|CastToSnowPlayerStateBP _array_element_2))
          (Variables|Default|SetComparePlayer _assnow_player_state_bp_3)
          (bind _score (Class|SnowGameState|GetScore (Variables|Default|GetSnowGameState) (Class|AdvancedSessionsLibrary|UniqueNetIdtoString (Class|AdvancedSessionsLibrary|GetUniqueNetIDfromPlayerState (Variables|Default|GetCurrentPlayer))) (Class|AdvancedSessionsLibrary|UniqueNetIdtoString (Class|AdvancedSessionsLibrary|GetUniqueNetIDfromPlayerState (Variables|Default|GetComparePlayer)))))
          (Variables|Default|SetCurrentScore (+ _score (Variables|Default|GetCurrentScore))))
        (if (> (Variables|Default|GetCurrentScore) (Utilities|Array|Get(acopy) (Variables|Default|GetHighestScores)))
          (Variables|Default|SetHighestScores (Utilities|Array|MakeArray (Variables|Default|GetCurrentScore)))
          (Variables|Default|SetHighestPlayers (Utilities|Array|MakeArray (Variables|Default|GetCurrentPlayer)))
          (elif (== (Variables|Default|GetCurrentScore) (Utilities|Array|Get(acopy) (Variables|Default|GetHighestScores)))
            (Utilities|Array|Add (Variables|Default|GetHighestScores) (Variables|Default|GetCurrentScore))
            (Utilities|Array|Add (Variables|Default|GetHighestPlayers) (Variables|Default|GetCurrentPlayer)))))
      (if (< (Utilities|Array|Length (Variables|Default|GetHighestScores)) 2)
        (Variables|Default|SetMatchText (Utilities|Text|ToText(String) (Utilities|String|Append "Player " (Utilities|String|ToString(Integer) (Variables|/Script/Engine.PlayerState|GetPlayerId (Utilities|Array|Get(acopy) (Variables|Default|GetHighestPlayers)))) "is the Winner!")))
        (else
          (Variables|Default|SetMatchText "Tie Game!")))))
  (Rendering|Components|TextRender|SetText (Variables|Default|GetTextRender) (Variables|Default|GetMatchText)))

(fn ConstructionScript)