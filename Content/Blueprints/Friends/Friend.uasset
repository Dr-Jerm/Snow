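; Friend actor that shows a text label and, when grabbed, invites that online friend to the player's session.
; Tick pushes the Text variable into the TextRender component whenever the two differ.
; BeGrabbed runs the parent grab logic, sends a session invite to FriendID with printed success or failure, then opens the invite UI for the first player controller.
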(event EventBeginPlay)

(event Collision|EventActorBeginOverlap
  (params (OtherActor :type Actor%20Object%20Reference)))

(event EventBeGrabbed
  (params (Grabber :type Pawn%20Object%20Reference) (Hand :type EControllerHand%20Enum :default "Left") (GrabLocation :type Vector))
  (bind _returnvalue (Game|GetPlayerController 0))
  (|CallParentFunction Grabber Hand GrabLocation)
  (Class|AdvancedFriendsLibrary|SendSessionInvitetoFriend _returnvalue (Variables|Default|GetfriendID)
    (:OnSuccess
      (Development|PrintText "Session invite sent!"))
    (:OnFailure
      (Development|PrintText "Session invite failed!")))
  (Class|AdvancedExternalUILibrary|ShowInviteUI _returnvalue))

(event EventTick
  (params (DeltaSeconds :type Float%20%28single-precision%29))
  (bind _text (Variables|Default|Gettext))
  (if (Utilities|Enum|NotEqual(Enum) _text (Utilities|String|ToString(Text) (Variables|/Script/Engine.TextRenderComponent|GetText (Variables|Default|GetTextRender))))
    (Rendering|Components|TextRender|SetText (Variables|Default|GetTextRender) (Utilities|Text|ToText(String) _text))))

(fn ConstructionScript)