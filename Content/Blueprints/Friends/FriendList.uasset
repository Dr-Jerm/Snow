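; FriendList is an actor that builds an in-world list of the player's Steam friends who are playing the same game.
; On every Tick it reads friends from SteamGameInstanceBP and adds a Friend child actor for each match, setting its display name and net ID.
; Entries stack along Z by OffsetSpacing, with no reset of the offset.
; The logic that destroys existing entries before rebuilding is unconnected, so entries accumulate each tick.
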(event EventBeginPlay)

(event Collision|EventActorBeginOverlap
  (params (OtherActor :type Actor%20Object%20Reference)))

(event EventTick
  (params (DeltaSeconds :type Float%20%28single-precision%29))
  (bind _assteam_game_instance_bp (Utilities|Casting|CastToSteamGameInstanceBP (Game|GetGameInstance)))
  (bind _friendslist (Default|GetFriends _assteam_game_instance_bp))
  (for _array_element _friendslist
    (if (.bIsPlayingSameGame (Utilities|Struct|BreakBPFriendInfo _array_element))
      (bind _returnvalue (AddComponent|AddChildActorComponent false (Math|Transform|MakeTransform (Math|Vector|MakeVector 0.0 0.0 (Variables|Default|Getoffset)))))
      (Utilities|Array|Add (Variables|Default|GetFriends) _returnvalue)
      (bind _asfriend (Utilities|Casting|CastToFriend (Variables|/Script/Engine.ChildActorComponent|GetChildActor _returnvalue)))
      (Variables|/Game/Blueprints/Friends/Friend.Friend_C|Settext _asfriend (.DisplayName (Utilities|Struct|BreakBPFriendInfo _array_element)))
      (Variables|/Game/Blueprints/Friends/Friend.Friend_C|SetfriendID _asfriend (.UniqueNetId (Utilities|Struct|BreakBPFriendInfo _array_element)))
      (Variables|Default|Setoffset (+ (Variables|Default|GetoffsetSpacing) (Variables|Default|Getoffset))))))

(fn ConstructionScript)