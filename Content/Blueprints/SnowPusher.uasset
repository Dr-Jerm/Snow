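; SnowPusher is a Blueprint that records snow pushes on the landscape into a heightfield render target.
; Its construction script creates a dynamic snow brush material and finds the Landscape actor tagged "ground".
; PushSnow converts the hit location into scaled landscape-local space, feeds it with size and strength to the brush, and draws that material into the render target.
; BeginPlay clears the render target to black.
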(event Custom|PushSnow
  (params (hit :type Hit%20Result%20Structure) (size :type Float%20%28single-precision%29) (strength :type Float%20%28single-precision%29))
  (Rendering|Material|SetScalarParameterValue (Variables|Default|GetSnowBrush_MID) "ForceSize" size :!class /Script/Engine.MaterialInstanceDynamic)
  (Rendering|Material|SetScalarParameterValue (Variables|Default|GetSnowBrush_MID) "ForceStrength" strength :!class /Script/Engine.MaterialInstanceDynamic)
  (Rendering|Material|SetVectorParameterValue (Variables|Default|GetSnowBrush_MID) "ForcePosition" (Math|Conversions|ToLinearColor(Vector) (/ (Math|Transform|TransformLocation (Math|Transform|InvertTransform (Transformation|GetActorTransform (Variables|Default|GetLandscapeRef))) (.Location (Collision|BreakHitResult hit))) 1e+03)) :!class /Script/Engine.MaterialInstanceDynamic)
  (Rendering|DrawMaterialtoRenderTarget (Variables|Default|GetHeightfield_RT) (Variables|Default|GetSnowBrush_MID)))

(event EventBeginPlay
  (Rendering|ClearRenderTarget2D (Variables|Default|GetHeightfield_RT)))

(event Collision|EventActorBeginOverlap
  (params (OtherActor :type Actor%20Object%20Reference)))

(event EventTick
  (params (DeltaSeconds :type Float%20%28single-precision%29)))

(fn ConstructionScript
  (CallFunction|GetLandscape)
  (bind _returnvalue (Rendering|Material|CreateDynamicMaterialInstance "/Game/Materials/M_SnowBrush.M_SnowBrush" :!class /Script/Engine.KismetMaterialLibrary))
  (Variables|Default|SetSnowBrush_MID _returnvalue))

(fn GetLandscape
  (bind _outactors (Actor|GetAllActorsOfClass "/Script/Landscape.Landscape"))
  (for _array_element _outactors
    (if (Actor|ActorHasTag _array_element "ground")
      (Variables|Default|SetLandscapeRef _array_element))))