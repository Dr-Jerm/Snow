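; A set of VR teleport helper functions for placing the player and validating landing spots.
; TeleportToActor requests a pawn teleport, subtracting rotated horizontal head offset and flattened head yaw so the head matches the target actor.
; GetTeleportToLocationRotation returns the same compensation for a location, using the pawn's own rotation.
; CheckForTeleportSurface traces down through WorldStatic objects for SnowGameStateBP's surface tag; its teleportIgnore check is disconnected.
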(fn TeleporttoActor
  (params (VRBaseBP :type VR%20Base%20BP%20Object%20Reference) (TargetActor :type Actor%20Object%20Reference))
  (bind _returnvalue (Transformation|GetActorRotation TargetActor))
  (bind _returnvalue_2 (Math|Vector|MakeVector 0.0 0.0 1.0))
  (bind _vrstatereplicated (Variables|/Script/Snow.VRBase|GetvrStateReplicated VRBaseBP))
  (bind (_headposition _headrotation) (Utilities|Struct|BreakVRState _vrstatereplicated))
  (bind (_x _y) (Math|Vector|BreakVector _headposition))
  (bind _returnvalue_3 (Math|Rotator|GetRotationXVector _headrotation))
  (bind (_x_2 _y_2) (Math|Vector|BreakVector _returnvalue_3))
  (bind _returnvalue_4 (Math|Vector|MakeVector _x_2 _y_2 0.0))
  (bind _returnvalue_5 (Math|Rotator|MakeRotfromXZ _returnvalue_4 _returnvalue_2))
  (bind _returnvalue_6 (Math|Rotator|Delta(Rotator) _returnvalue _returnvalue_5))
  (Default|RequestTeleport VRBaseBP (- (Transformation|GetActorLocation TargetActor) (Math|Vector|RotateVector (Math|Vector|MakeVector _x _y 0.0) _returnvalue_6)) _returnvalue_6))

(fn CheckforTeleportSurface
  (params (Location :type Vector))
  (bind _outhits (Class|KismetSystemLibrary|LineTraceMultiforObjects 0 (+ Location "0, 0,5.000000") (+ Location "0, 0,-500.000000") (Utilities|Array|MakeArray "ObjectTypeQuery1") false 0 "None" true))
  (for _array_element _outhits
    (bind _assnow_game_state_bp (Utilities|Casting|CastToSnowGameStateBP (Game|GetGameState))
      (:then
        (if (Actor|ActorHasTag (.HitActor (Collision|BreakHitResult _array_element)) (Variables|/Game/GameModes/SnowGameStateBP.SnowGameStateBP_C|GetTagTeleportSurface _assnow_game_state_bp))
          (return true)))
      (:CastFailed
        (return false))))
  (return false))

(fn GetTeleporttoLocationRotation
  (params (Location :type Vector) (VRPawn :type VR%20Base%20BP%20Object%20Reference))
  (bind _returnvalue (Transformation|GetActorRotation VRPawn))
  (bind _returnvalue_2 (Math|Vector|MakeVector 0.0 0.0 1.0))
  (bind _vrstatereplicated (Variables|/Script/Snow.VRBase|GetvrStateReplicated VRPawn))
  (bind (_headposition _headrotation) (Utilities|Struct|BreakVRState _vrstatereplicated))
  (bind (_x _y) (Math|Vector|BreakVector _headposition))
  (bind _returnvalue_3 (Math|Rotator|GetRotationXVector _headrotation))
  (bind (_x_2 _y_2) (Math|Vector|BreakVector _returnvalue_3))
  (bind _returnvalue_4 (Math|Vector|MakeVector _x_2 _y_2 0.0))
  (bind _returnvalue_5 (Math|Rotator|MakeRotfromXZ _returnvalue_4 _returnvalue_2))
  (bind _returnvalue_6 (Math|Rotator|Delta(Rotator) _returnvalue _returnvalue_5))
  (return (- Location (Math|Vector|RotateVector (Math|Vector|MakeVector _x _y 0.0) _returnvalue_6)) _returnvalue_6))