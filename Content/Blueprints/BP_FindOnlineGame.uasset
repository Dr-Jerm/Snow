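; Grabbable matchmaking object that puts the player into an online or LAN match when grabbed.
; With LAN enabled in the lanConfig file, it either opens BRL_rag as a listen server or connects to the configured server.
; Otherwise it starts a session search through the Steam game instance and plays force feedback for the grabbing hand.
; Tick polls the search state, joining the best session or hosting BRL_rag if none is found.
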(event EventBeginPlay)

(event EventTick
  (params (DeltaSeconds :type Float%20%28single-precision%29))
  (if (Variables|Default|GetwaitingToJoin)
    (bind _assteam_game_instance_bp (Utilities|Casting|CastToSteamGameInstanceBP (Game|GetGameInstance)))
    (switch Utilities|FlowControl|Switch|SwitchonE_OnlineState (Variables|/Game/Online/SteamGameInstanceBP.SteamGameInstanceBP_C|GetCurrentOnlineState _assteam_game_instance_bp)
      (:NewEnumerator0
        (Variables|Default|SetwaitingToJoin false :!label _label)
        (Development|PrintText (Utilities|Text|FormatText "Error: {error}" (Utilities|Text|ToText(String) (Variables|/Game/Online/SteamGameInstanceBP.SteamGameInstanceBP_C|GetErrorMessage _assteam_game_instance_bp))) true true "(R=1.000000,G=0.025124,B=0.000000,A=1.000000)"))
      (:NewEnumerator2
        (bind _foundsession (Default|SelectBestSession _assteam_game_instance_bp))
        (if (Class|AdvancedSessionsLibrary|IsValidSession _foundsession)
          (Default|JoinSession _assteam_game_instance_bp _foundsession)
          (Variables|Default|SetwaitingToJoin false)
          (else
            (Default|HostGame _assteam_game_instance_bp "BRL_rag" :!label _label_2)
            (goto _label))))
      (:NewEnumerator7
        (goto _label_2))
      (:NewEnumerator3
        (goto _label))
      (:NewEnumerator4
        (goto _label))
      (:NewEnumerator5
        (goto _label))
      (:NewEnumerator6
        (goto _label)))))

(event EventBeGrabbed
  (params (Grabber :type Pawn%20Object%20Reference) (Hand :type EControllerHand%20Enum :default "Left") (GrabLocation :type Vector))
  (|CallParentFunction Grabber Hand GrabLocation)
  (bind _assteam_game_instance_bp (Utilities|Casting|CastToSteamGameInstanceBP (Game|GetGameInstance)))
  (if (Class|ConfigLibrary|ReadConfigBoolValue "lanConfig" "bEnabled")
    (if (Class|ConfigLibrary|ReadConfigBoolValue "lanConfig" "bIsServer")
      (Game|OpenLevel(byName) "BRL_rag" true "listen?bIsLanMatch=1")
      (else
        (Development|ExecuteConsoleCommand (Utilities|String|Append "open " (Class|ConfigLibrary|ReadConfigStringValue "lanConfig" "server")))))
    (else
      (switch Utilities|FlowControl|Switch|SwitchonE_OnlineState (Variables|/Game/Online/SteamGameInstanceBP.SteamGameInstanceBP_C|GetCurrentOnlineState _assteam_game_instance_bp)
        (:NewEnumerator0
          _)
        (:NewEnumerator7
          _)
        (:NewEnumerator5
          _))
      (Default|FindSessions _assteam_game_instance_bp false)
      (Variables|Default|SetwaitingToJoin true)
      (bind _asplayer_controller (Utilities|Casting|CastToPlayerController (Pawn|GetController Grabber)))
      (switch Utilities|FlowControl|Switch|SwitchonEControllerHand Hand
        (:Left
          (Game|Feedback|ClientPlayForceFeedback _asplayer_controller "/Game/ForceFeedback/SnowballHitLeft.SnowballHitLeft" false "None"))
        (:Right
          (Game|Feedback|ClientPlayForceFeedback _asplayer_controller "/Game/ForceFeedback/SnowballHitRight.SnowballHitRight" false "None"))))))

(fn ConstructionScript)