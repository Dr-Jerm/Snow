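; RapidMoveTo is a Behavior Tree task that moves an AI follower's pawn to the actor stored in the TargetToFollow blackboard key.
; It casts the owner to Follower_AI_CON and caches the controller on first execution, then runs AIMoveTo with zero acceptance radius.
; The task finishes successfully when the move succeeds, with no handling for a failed move or failed cast.
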(event EventReceiveExecute
  (params (OwnerActor :type Actor%20Object%20Reference))
  (if (!= (Variables|Default|GetAI%20CON%20Ref) 0)
    _
    (else
      (bind _asfollower_ai_con (Utilities|Casting|CastToFollower_AI_CON OwnerActor))
      (Variables|Default|SetAI%20CON%20Ref _asfollower_ai_con)))
  (AI|AIMoveTo (Pawn|GetControlledPawn (Variables|Default|GetAI%20CON%20Ref)) "0, 0, 0" (AI|BehaviorTree|GetBlackboardValueasActor (Variables|Default|GetTargetToFollow)) 0.0 false
    (:OnSuccess
      (AI|BehaviorTree|FinishExecute true))))