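; Behavior tree aggro check that, each tick, looks for visible targets around a Follower_AI_CON's pawn.
; A multi-sphere trace ignoring AI_Characters gathers nearby TargetableInterface actors, then a Camera-channel line trace toward each one's targetable location tests line of sight.
; Visible targets set TargetToFollow and TargetLocation on the blackboard; blocked ones clear TargetToFollow and TargetToHit, so the last candidate wins.
; Debug prints and lines show each candidate.
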(event Custom|ServerReceiveTick
  (params (OwnerActor :type Actor%20Object%20Reference) (DeltaSeconds :type Float%20%28single-precision%29))
  (if (!= (Variables|Default|GetAI%20CON%20Ref) 0)
    _
    (else
      (bind _asfollower_ai_con (Utilities|Casting|CastToFollower_AI_CON OwnerActor))
      (Variables|Default|SetAI%20CON%20Ref _asfollower_ai_con)))
  (bind _outactors (Actor|GetAllActorsOfClass "/Game/Blueprints/BaseAI/AI_Character.AI_Character_C"))
  (Variables|Default|SetMyLocation (Transformation|GetActorLocation (Pawn|GetControlledPawn (Variables|Default|GetAI%20CON%20Ref))))
  (bind _outhits (Collision|MultiSphereTraceForObjects (Transformation|GetActorLocation (Pawn|GetControlledPawn (Variables|Default|GetAI%20CON%20Ref))) (+ (Transformation|GetActorLocation (Pawn|GetControlledPawn (Variables|Default|GetAI%20CON%20Ref))) "0, 0,15.000000") 1.5e+03 (Variables|Default|GetDesiredObjectTypes) false _outactors "None"))
  (bind _array_element (Utilities|Array|ForEachLoopwithBreak _outhits)
    (:LoopBody
      (if (Utilities|DoesObjectImplementInterface (.HitActor (Collision|BreakHitResult _array_element)) "/Game/TargetableInterface.TargetableInterface_C")
        (Development|PrintString (Utilities|GetDisplayName (.HitActor (Collision|BreakHitResult _array_element))))
        (bind _location (Class|TargetableInterface|GetTargetableLocation(Message) (.HitActor (Collision|BreakHitResult _array_element))))
        (Rendering|Debug|DrawDebugLine (Variables|Default|GetMyLocation) (+ (Variables|Default|GetMyLocation) (* (Class|KismetMathLibrary|GetDirectionVector (Variables|Default|GetMyLocation) _location) 2e+03)) "(R=1.000000,G=0.016751,B=0.000000,A=1.000000)" 1.0 1.0)
        (bind _outhit (Collision|LineTraceByChannel (Variables|Default|GetMyLocation) (+ (Variables|Default|GetMyLocation) (* (Class|KismetMathLibrary|GetDirectionVector (Variables|Default|GetMyLocation) _location) 2e+03)) "TraceTypeQuery2" false _outactors "None"))
        (if (== (.HitActor (Collision|BreakHitResult _outhit)) (.HitActor (Collision|BreakHitResult _array_element)))
          (Class|BTFunctionLibrary|SetBlackboardValueasObject (Variables|Default|GetTargetToFollow) (.HitActor (Collision|BreakHitResult _outhit)))
          (AI|BehaviorTree|SetBlackboardValueasVector (Variables|Default|GetTargetLocation) (Transformation|GetActorLocation (.HitActor (Collision|BreakHitResult _outhit))))
          (else
            (Class|BTFunctionLibrary|SetBlackboardValueasObject (Variables|Default|GetTargetToFollow))
            (Class|BTFunctionLibrary|SetBlackboardValueasObject (Variables|Default|GetTargetToHit))))))))

(event EventTick
  (params (OwnerActor :type Actor%20Object%20Reference) (DeltaSeconds :type Float%20%28single-precision%29))
  (CallFunction|ServerReceiveTick OwnerActor DeltaSeconds))