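; AI character for a snow person that can be targeted and knocked down by hits.
; Each tick, the locally controlled instance passes its location to BroadcastPosition, which sets the actor's location directly as a simple manual position sync.
; BroadcastOnHit switches the mesh to a simulated ragdoll, then destroys the actor after a short delay.
; GetTargetableLocation exposes the capsule's world location as the target point.
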(event EventBeginPlay)

(event Collision|EventActorBeginOverlap
  (params (OtherActor :type Actor%20Object%20Reference)))

(event EventTick
  (params (DeltaSeconds :type Float%20%28single-precision%29))
  (if (Pawn|IsLocallyControlled)
    (CallFunction|BroadcastPosition (Transformation|GetActorLocation))))

(event Custom|BroadcastPosition
  (params (ServerLocation :type Vector))
  (Transformation|SetActorLocation ServerLocation false false))

(event Custom|BroadcastOnHit
  (bind _mesh (Variables|Character|GetMesh))
  (Collision|SetCollisionProfileName _mesh "Ragdoll" :!class /Script/Engine.PrimitiveComponent)
  (Components|SkinnedMesh|SetPhysicsAsset (Variables|Character|GetMesh) "/Game/Assets/snowman/SnowPersonPhysicsRagdoll.SnowPersonPhysicsRagdoll" false)
  (Physics|SetSimulatePhysics _mesh true)
  (Utilities|FlowControl|Delay 3.0)
  (Actor|DestroyActor))

(fn ConstructionScript)

(fn GetTargetableLocation
  (return (Transformation|GetWorldLocation (Variables|Collision|GetCapsuleComponent))))