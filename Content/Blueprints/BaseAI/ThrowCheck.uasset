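; Behavior tree tick node for Follower_AI_CON that finds visible targetable actors around the AI and writes them to the blackboard.
; A sphere trace around the pawn gathers TargetableInterface actors, ignoring all AI_Characters.
; A Camera-channel line trace toward each one's targetable location confirms line of sight.
; Each check sets or clears TargetToHit, TargetToFollow and TargetLocation, so the last candidate checked wins.
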(event Custom|ServerReceiveTick
  (params (OwnerActor :type Actor%20Object%20Reference) (DeltaSeconds :type Float%20%28single-precision%29))
  (if (!= (Variables|Default|GetAI%20CON%20Ref) 0)
    _
    (else
      (bind _asfollower_ai_con (Utilities|Casting|CastToFollower_AI_CON OwnerActor))
      (Variables|Default|SetAI%20CON%20Ref _asfollower_ai_con)))
  (bind _outactors (Actor|GetAllActorsOfClass "/Game/Blueprints/BaseAI/AI_Character.AI_Character_C"))
  (Variables|Default|SetMyLocation (Transformation|GetActorLocation (Pawn|GetControlledPawn (Variables|Default|GetAI%20CON%20Ref))))
  (bind _outhits (Collision|MultiSphereTraceForObjects (Transformation|GetActorLocation (Pawn|GetControlledPawn (Variables|Default|GetAI%20CON%20Ref))) (+ (Transformation|GetActorLocation (Pawn|GetControlledPawn (Variables|Default|GetAI%20CON%20Ref))) "0, 0,15.000000") 1.5e+03 (Variables|Default|GetDesiredObjectTypes) false _outactors "None"))
  (bind _array_element (Utilities|Array|ForEachLoopwithBreak _outhits)
    (:LoopBody
      (if (Utilities|DoesObjectImplementInterface (.HitActor (Collision|BreakHitResult _array_element)) "/Game/TargetableInterface.TargetableInterface_C")
        (bind _location (Class|TargetableInterface|GetTargetableLocation(Message) (.HitActor (Collision|BreakHitResult _array_element))))
        (bind _outhit (Collision|LineTraceByChannel (Variables|Default|GetMyLocation) (+ (Variables|Default|GetMyLocation) (* (Class|KismetMathLibrary|GetDirectionVector (Variables|Default|GetMyLocation) _location) 2e+03)) "TraceTypeQuery2" false _outactors "None"))
        (if (== (.HitActor (Collision|BreakHitResult _outhit)) (.HitActor (Collision|BreakHitResult _array_element)))
          (Class|BTFunctionLibrary|SetBlackboardValueasObject (Variables|Default|GetTargetToHit) (.HitActor (Collision|BreakHitResult _outhit)))
          (Class|BTFunctionLibrary|SetBlackboardValueasObject (Variables|Default|GetTargetToFollow) (.HitActor (Collision|BreakHitResult _outhit)))
          (AI|BehaviorTree|SetBlackboardValueasVector (Variables|Default|GetTargetLocation) (Transformation|GetActorLocation (.HitActor (Collision|BreakHitResult _outhit))))
          (else
            (Class|BTFunctionLibrary|SetBlackboardValueasObject (Variables|Default|GetTargetToHit))
            (Class|BTFunctionLibrary|SetBlackboardValueasObject (Variables|Default|GetTargetToFollow))
            (AI|BehaviorTree|SetBlackboardValueasVector (Variables|Default|GetTargetLocation) "0, 0, 0")))))))

(event EventTick
  (params (OwnerActor :type Actor%20Object%20Reference) (DeltaSeconds :type Float%20%28single-precision%29))
  (CallFunction|ServerReceiveTick OwnerActor DeltaSeconds))