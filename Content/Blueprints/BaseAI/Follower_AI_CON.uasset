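; AI controller for follower characters that runs the FollowerBT behavior tree on the FollowerBlackboard.
; BeginPlay sets up the blackboard and, if a pawn is possessed, stores its location as HomeLocation and starts the tree.
; Tick repeats the home write and tree start while HasInitializedHome is false, and sets that flag to false afterward, so this branch never latches off by itself.
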(event EventBeginPlay
  (bind _returnvalue (Pawn|GetControlledPawn))
  (Class|AIController|UseBlackboard "/Game/Blueprints/BaseAI/FollowerBlackboard.FollowerBlackboard")
  (if (Utilities|IsValid _returnvalue)
    (AI|Components|Blackboard|SetValueasVector (AI|GetBlackboard self) (Variables|Default|GetHomeLocation) (Transformation|GetActorLocation _returnvalue))
    (AI|RunBehaviorTree "/Game/Blueprints/BaseAI/FollowerBT.FollowerBT")))

(event EventTick
  (params (DeltaSeconds :type Float%20%28single-precision%29))
  (if (not (Variables|Default|GethasInitializedHome))
    (AI|Components|Blackboard|SetValueasVector (AI|GetBlackboard self) (Variables|Default|GetHomeLocation) (Transformation|GetActorLocation (Pawn|GetControlledPawn)))
    (AI|RunBehaviorTree "/Game/Blueprints/BaseAI/FollowerBT.FollowerBT")
    (Variables|Default|SethasInitializedHome false)))

(fn ConstructionScript)