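; InThrowRange is a Behavior Tree condition for follower AI that checks whether the pawn is close enough to throw at its target.
; It casts the owner to Follower_AI_CON and measures the distance from the controlled pawn to the actor in the TargetToHit blackboard key.
; The condition passes when that distance is within AcceptableDistance.
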(fn PerformConditionCheck
  (params (OwnerActor :type Actor%20Object%20Reference))
  (bind _asfollower_ai_con (Utilities|Casting|CastToFollower_AI_CON OwnerActor))
  (Variables|Default|SetAI%20CON%20Ref _asfollower_ai_con)
  (return (<= (Math|Vector|VectorLength (- (Transformation|GetActorLocation (Pawn|GetControlledPawn (Variables|Default|GetAI%20CON%20Ref))) (Transformation|GetActorLocation (AI|BehaviorTree|GetBlackboardValueasActor (Variables|Default|GetTargetToHit))))) (Variables|Default|GetAcceptableDistance))))