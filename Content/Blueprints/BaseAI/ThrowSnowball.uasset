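; Behavior tree task that makes a follower AI character throw a snowball at the blackboard's TargetToHit actor.
; A server-time cooldown gates each throw, and the task finishes successfully whether it throws or skips.
; A kinematics helper solves a fixed-flight-time arc under gravity from the throw socket to the target's targetable location.
; FireSnowball, in the Server graph, spawns the replicated snowball and launches it with physics.
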(event EventReceiveExecute
  (params (OwnerActor :type Actor%20Object%20Reference))
  (bind _returnvalue (Game|GetGameState))
  (bind _returnvalue_2 (GameState|GetServerWorldTimeSeconds _returnvalue))
  (if (!= (Variables|Default|GetAI%20CON%20Ref) 0)
    _
    (else
      (bind _asfollower_ai_con (Utilities|Casting|CastToFollower_AI_CON OwnerActor))
      (Variables|Default|SetAI%20CON%20Ref _asfollower_ai_con)))
  (bind _location (Class|TargetableInterface|GetTargetableLocation(Message) (AI|BehaviorTree|GetBlackboardValueasActor (Variables|Default|GetTargetToHit))))
  (if (> (Math|Float|Absolute(Float) (- _returnvalue_2 (Variables|Default|GetPreviousReleasedTime))) 2.5)
    (Variables|Default|SetPreviousReleasedTime _returnvalue_2)
    (bind _asai_character (Utilities|Casting|CastToAI_Character (Pawn|GetControlledPawn (Variables|Default|GetAI%20CON%20Ref))))
    (CallFunction|FireSnowball (Pawn|GetControlledPawn (Variables|Default|GetAI%20CON%20Ref)) (Class|KinematicsFunctionLibrary|KinematicsCalculateInitialVelocity (Transformation|GetSocketLocation (Variables|/Script/Engine.Character|GetMesh _asai_character) "ThrowSocket") _location "0.000000, 0,-980.000000" 0.75) (Transformation|GetSocketLocation (Variables|/Script/Engine.Character|GetMesh _asai_character) "ThrowSocket") (GameState|GetServerWorldTimeSeconds (Game|GetGameState))))
  (AI|BehaviorTree|FinishExecute true))

(event Custom|FireSnowball
  (params (Releaser :type Pawn%20Object%20Reference) (Velocity :type Vector) (Location :type Vector) (ReleasedTime :type Float%20%28single-precision%29))
  (Variables|Default|SetReleaser Releaser)
  (Variables|Default|SetInitialVelocity Velocity)
  (Variables|Default|SetInitialPosition Location)
  (Variables|Default|SetPreviousReleasedTime ReleasedTime)
  (bind _returnvalue (Game|SpawnActorfromClass "/Game/Assets/Snowball/ASnowball_replicated.ASnowball_replicated_C" (Math|Transform|MakeTransform (Variables|Default|GetInitialPosition)) "Undefined" (Variables|Default|GetReleaser) (Variables|Default|GetReleaser)))
  (Physics|SetSimulatePhysics (Variables|/Game/Throwable.Throwable_C|GetPhysicsComponent _returnvalue) true)
  (Collision|SetCollisionProfileName (Variables|/Game/Throwable.Throwable_C|GetPhysicsComponent _returnvalue) "None" :!class /Script/Engine.PrimitiveComponent)
  (Physics|SetPhysicsLinearVelocity (Variables|/Game/Throwable.Throwable_C|GetPhysicsComponent _returnvalue) (Variables|Default|GetInitialVelocity) false "None")
  (Class|PrimitiveComponent|WakeRigidBody (Variables|/Game/Throwable.Throwable_C|GetPhysicsComponent _returnvalue) "None"))