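; ProceduralPlane is an actor that builds a single rectangular plane with a configurable size, material and axis-aligned facing direction.
; The construction script switches on FaceDirection to set the four vertices and normals for one of six directions and resizes a Box component to match.
; It then creates the ProceduralMesh section from those arrays plus the Triangles and UVs variables, and applies the material.
; The event graph holds no logic.
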(event EventBeginPlay)

(event Collision|EventActorBeginOverlap
  (params (OtherActor :type Actor%20Object%20Reference)))

(event EventTick
  (params (DeltaSeconds :type Float%20%28single-precision%29)))

(fn ConstructionScript
  (bind _proceduralmesh (Variables|Default|GetProceduralMesh))
  (bind _size (Variables|Plane|GetSize))
  (bind _size_2 (Variables|Plane|GetSize))
  (bind _size_3 (Variables|Plane|GetSize))
  (bind _size_4 (Variables|Plane|GetSize))
  (bind _size_5 (Variables|Plane|GetSize))
  (bind _size_6 (Variables|Plane|GetSize))
  (bind _returnvalue (* (.x _size) -1.0))
  (bind _returnvalue_2 (* (.y _size) -1.0))
  (bind _returnvalue_3 (* (.x _size_2) -1.0))
  (bind _returnvalue_4 (* (.y _size_2) -1.0))
  (bind _returnvalue_5 (* (.x _size_3) -1.0))
  (bind _returnvalue_6 (* (.y _size_3) -1.0))
  (bind _returnvalue_7 (* (.x _size_4) -1.0))
  (bind _returnvalue_8 (* (.y _size_4) -1.0))
  (bind _returnvalue_9 (* (.x _size_5) -1.0))
  (bind _returnvalue_10 (* (.y _size_5) -1.0))
  (bind _returnvalue_11 (* (.x _size_6) -1.0))
  (bind _returnvalue_12 (* (.y _size_6) -1.0))
  (Utilities|FlowControl|Sequence
    (:then_0
      (switch Utilities|FlowControl|Switch|SwitchonEProceduralPlaneDirection (Variables|Plane|GetFaceDirection)
        (:NewEnumerator0
          (Variables|Default|SetVertices (Utilities|Array|MakeArray (Math|Vector|MakeVector 0.0 _returnvalue_3 (.y _size_2)) (Math|Vector|MakeVector 0.0 (.x _size_2) (.y _size_2)) (Math|Vector|MakeVector 0.0 _returnvalue_3 _returnvalue_4) (Math|Vector|MakeVector 0.0 (.x _size_2) _returnvalue_4)))
          (Variables|Default|SetNormals (Utilities|Array|MakeArray "1.000000,0.000000,0.000000" "1.000000,0.000000,0.000000" "1.000000,0.000000,0.000000" "1.000000,0,0"))
          (Components|Box|SetBoxExtent (Variables|Default|GetBox) (Math|Vector|MakeVector 0.1 (.x _size_2) (.y _size_2)) true))
        (:NewEnumerator1
          (Variables|Default|SetVertices (Utilities|Array|MakeArray (Math|Vector|MakeVector (.x _size_5) 0.0 (.y _size_5)) (Math|Vector|MakeVector _returnvalue_9 0.0 (.y _size_5)) (Math|Vector|MakeVector (.x _size_5) 0.0 _returnvalue_10) (Math|Vector|MakeVector _returnvalue_9 0.0 _returnvalue_10)))
          (Variables|Default|SetNormals (Utilities|Array|MakeArray "0.000000,1.000000,0.000000" "0.000000,1.000000,0.000000" "0.000000,1.000000,0.000000" "0.000000,1.000000,0.000000"))
          (Components|Box|SetBoxExtent (Variables|Default|GetBox) (Math|Vector|MakeVector (.x _size_5) 0.0 (.y _size_5)) true))
        (:NewEnumerator2
          (Variables|Default|SetVertices (Utilities|Array|MakeArray (Math|Vector|MakeVector (.x _size_6) _returnvalue_12 0.0) (Math|Vector|MakeVector _returnvalue_11 _returnvalue_12 0.0) (Math|Vector|MakeVector (.x _size_6) (.y _size_6) 0.0) (Math|Vector|MakeVector _returnvalue_11 (.y _size_6) 0.0)))
          (Variables|Default|SetNormals (Utilities|Array|MakeArray "0.000000,0.000000,1.000000" "0.000000,0.000000,1.000000" "0.000000,0.000000,1.000000" "0.000000,0.000000,1.000000"))
          (Components|Box|SetBoxExtent (Variables|Default|GetBox) (Math|Vector|MakeVector (.x _size_6) (.y _size_6) 0.0) true))
        (:NewEnumerator3
          (Variables|Default|SetVertices (Utilities|Array|MakeArray (Math|Vector|MakeVector 0.0 (.x _size_3) (.y _size_3)) (Math|Vector|MakeVector 0.0 _returnvalue_5 (.y _size_3)) (Math|Vector|MakeVector 0.0 (.x _size_3) _returnvalue_6) (Math|Vector|MakeVector 0.0 _returnvalue_5 _returnvalue_6)))
          (Variables|Default|SetNormals (Utilities|Array|MakeArray "-1.000000,0.000000,0.000000" "-1.000000,0.000000,0.000000" "-1.000000,0.000000,0.000000" "-1.000000,0.000000,0.000000"))
          (Components|Box|SetBoxExtent (Variables|Default|GetBox) (Math|Vector|MakeVector 0.1 (.x _size_3) (.y _size_3)) true))
        (:NewEnumerator4
          (Variables|Default|SetVertices (Utilities|Array|MakeArray (Math|Vector|MakeVector _returnvalue 0.0 (.y _size)) (Math|Vector|MakeVector (.x _size) 0.0 (.y _size)) (Math|Vector|MakeVector _returnvalue 0.0 _returnvalue_2) (Math|Vector|MakeVector (.x _size) 0.0 _returnvalue_2)))
          (Variables|Default|SetNormals (Utilities|Array|MakeArray "0.000000,-1.000000,0.000000" "0.000000,-1.000000,0.000000" "0.000000,-1.000000,0.000000" "0.000000,-1.000000,0.000000"))
          (Components|Box|SetBoxExtent (Variables|Default|GetBox) (Math|Vector|MakeVector (.x _size) 0.0 (.y _size)) true))
        (:NewEnumerator5
          (Variables|Default|SetVertices (Utilities|Array|MakeArray (Math|Vector|MakeVector (.x _size_4) (.y _size_4) 0.0) (Math|Vector|MakeVector _returnvalue_7 (.y _size_4) 0.0) (Math|Vector|MakeVector (.x _size_4) _returnvalue_8 0.0) (Math|Vector|MakeVector _returnvalue_7 _returnvalue_8 0.0)))
          (Variables|Default|SetNormals (Utilities|Array|MakeArray "0.000000,0.000000,-1.000000" "0.000000,0.000000,-1.000000" "0.000000,0.000000,-1.000000" "0.000000,0.000000,-1.000000"))
          (Components|Box|SetBoxExtent (Variables|Default|GetBox) (Math|Vector|MakeVector (.x _size_4) (.y _size_4) 0.0) true))))
    (:then_1
      (Class|ProceduralMeshComponent|CreateMeshSection _proceduralmesh 0 (Variables|Default|GetVertices) (Variables|Default|GetTriangles) (Variables|Default|GetNormals) (Variables|Default|GetUVs) 0 0 false)
      (Rendering|Material|SetMaterial _proceduralmesh 0 (Variables|Plane|GetMaterial)))))