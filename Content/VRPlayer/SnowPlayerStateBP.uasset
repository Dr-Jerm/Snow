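; SnowPlayerStateBP is a player state in the VR player folder that holds each player's API-sourced player data.
; A successful post-player callback casts the given controller's player state to this class and stores the returned player in ApiPlayer.
; ApiPlayer uses RepNotify to call VisualChange on the referenced pawn, if valid, so its appearance follows the data.
; A failed post prints the response code, URL and JSON payload.
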(event EventBeginPlay)

(event EventTick
  (params (DeltaSeconds :type Float%20%28single-precision%29)))

(event EventPostPlayerComplete
  (params (player :type Snow%20API-player%20Struct%20Structure) (PlayerController :type Player%20Controller%20Object%20Reference))
  (bind _asbase_player_controller_bp (Utilities|Casting|CastToBasePlayerControllerBP PlayerController))
  (bind _assnow_player_state_bp (Utilities|Casting|CastToSnowPlayerStateBP (Variables|/Script/Engine.Controller|GetPlayerState _asbase_player_controller_bp)))
  (Variables|SnowPlayerStateBP_C|SetapiPlayer _assnow_player_state_bp player))

(event EventPostPlayerFail
  (params (responseCode :type Integer) (url :type String) (payload :type Va%20Rest%20Json%20Object%20Object%20Reference) (PlayerController :type Player%20Controller%20Object%20Reference))
  (Development|PrintText (Utilities|Text|ToText(String) (Utilities|String|Append "Response code: " (Utilities|String|ToString(Integer) responseCode) " URL: " url " Response: " (Class|VaRestJsonObject|EncodeJsontoSingleString payload)))))

(fn ConstructionScript)

(fn OnRepApiPlayer
  (bind _pawnreference (Variables|Default|GetpawnReference))
  (Utilities|IsValid _pawnreference
    (:Is%20Valid
      (Default|VisualChange _pawnreference))))