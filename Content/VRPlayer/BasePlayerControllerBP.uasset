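; Base VR player controller that handles debug-style hotkeys for travel, multiplayer matchmaking and voice chat.
; Keys 1 and 2 leave the session for fixed levels; key 3 either uses a LAN config to listen-host or connect, or finds/hosts sessions by the Steam GameInstance's online state, retrying on error.
; On client post-login, the local controller enables the HMD, sets Game-and-UI input and starts voice, which V toggles.
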(event EventBeginPlay)

(event EventTick
  (params (DeltaSeconds :type Float%20%28single-precision%29)))

(event Input|KeyboardEvents|V
  (params (Key :type Key%20Structure :default "AnyKey"))
  (:Pressed
    (Default|Toggle (Variables|Default|GetVoiceComponent))))

(event Input|KeyboardEvents|1
  (params (Key :type Key%20Structure :default "AnyKey"))
  (:Pressed
    (bind _assteam_game_instance_bp (Utilities|Casting|CastToSteamGameInstanceBP (Game|GetGameInstance)))
    (Default|LeaveSession _assteam_game_instance_bp "SNW_entry")))

(event Input|KeyboardEvents|2
  (params (Key :type Key%20Structure :default "AnyKey"))
  (:Pressed
    (bind _assteam_game_instance_bp (Utilities|Casting|CastToSteamGameInstanceBP (Game|GetGameInstance)))
    (Default|LeaveSession _assteam_game_instance_bp "TUT_basics")))

(event Input|KeyboardEvents|3
  (params (Key :type Key%20Structure :default "AnyKey"))
  (:Pressed
    (bind _assteam_game_instance_bp (Utilities|Casting|CastToSteamGameInstanceBP (Game|GetGameInstance)))
    (if (Class|ConfigLibrary|ReadConfigBoolValue "lanConfig" "bEnabled")
      (if (Class|ConfigLibrary|ReadConfigBoolValue "lanConfig" "bIsServer")
        (Game|OpenLevel(byName) "BRL_rag" true "listen?bIsLanMatch=1")
        (else
          (Development|ExecuteConsoleCommand (Utilities|String|Append "open " (Class|ConfigLibrary|ReadConfigStringValue "lanConfig" "server")))))
      (else
        (switch Utilities|FlowControl|Switch|SwitchonE_OnlineState (Variables|/Game/Online/SteamGameInstanceBP.SteamGameInstanceBP_C|GetCurrentOnlineState _assteam_game_instance_bp)
          (:NewEnumerator0
            (Default|FindSessions _assteam_game_instance_bp true :!label _label))
          (:NewEnumerator7
            (Default|HostGame _assteam_game_instance_bp "BRL_rag"))
          (:NewEnumerator5
            (Development|PrintText (Utilities|Text|FormatText "Error: {error}" (Utilities|Text|ToText(String) (Variables|/Game/Online/SteamGameInstanceBP.SteamGameInstanceBP_C|GetErrorMessage _assteam_game_instance_bp))) true true "(R=1.000000,G=0.025124,B=0.000000,A=1.000000)")
            (goto _label)))))))

(event Custom|ClientPostLogin
  (Development|PrintText "Client::PostLogin Called")
  (if (Pawn|IsLocalPlayerController)
    (Class|HeadMountedDisplayFunctionLibrary|EnableHMD true)
    (Input|SetInputModeGameandUI 0 0 false true)
    (Default|StartVoice (Variables|Default|GetVoiceComponent))))

(fn ConstructionScript)