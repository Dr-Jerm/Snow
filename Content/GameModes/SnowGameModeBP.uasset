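; Game mode for the multiplayer VR Snow game that signs players in through a backend player API and spawns them.
; On login or seamless travel, the server fetches the player record, posting a new one on 404 or using a local identity on -1.
; ConfirmPlayer possesses a new VRBaseBP at round-robin PlayerStarts, stores API data and assigns score index and color via game state.
; First-boot tutorial logic is disconnected.
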(event EventSeamlessTravelPlayer
  (params (Controller :type Controller%20Object%20Reference))
  (bind _asplayer_controller (Utilities|Casting|CastToPlayerController Controller))
  (Networking|SwitchHasAuthority
    (:Authority
      (Default|GetPlayer (Variables|Default|GetsnowAPI-player) _asplayer_controller))))

(event EventPostLogin
  (params (NewPlayer :type Player%20Controller%20Object%20Reference))
  (if (and (Class|ConfigLibrary|ReadConfigBoolValue "snow" "firstBoot") (not (Networking|IsDedicatedServer)))
    _
    (else
      _))
  (Networking|SwitchHasAuthority
    (:Authority
      (Default|GetPlayer (Variables|Default|GetsnowAPI-player) NewPlayer))))

(event EventTick
  (params (DeltaSeconds :type Float%20%28single-precision%29)))

(event EventOnSetMatchState
  (params (NewState :type Name)))

(event EventPostPlayerComplete
  (params (player :type Snow%20API-player%20Struct%20Structure) (PlayerController :type Player%20Controller%20Object%20Reference))
  (Utilities|IsValid PlayerController
    (:Is%20Valid
      (bind _asbase_player_controller_bp (Utilities|Casting|CastToBasePlayerControllerBP PlayerController)
        (:then
          (CallFunction|ConfirmPlayer _asbase_player_controller_bp player))
        (:CastFailed
          (Development|PrintText "ERROR: LOGIN FAILED" false :!label _label)
          (Game|QuitGame 0 "Quit"))))
    (:Is%20Not%20Valid
      (goto _label))))

(event EventBeginPlay
  (Development|ExecuteConsoleCommand "r.SetRes 2160x1200")
  (Variables|Default|SetServerTravelling false))

(event EventGetPlayerComplete
  (params (player :type Snow%20API-player%20Struct%20Structure) (PlayerController :type Player%20Controller%20Object%20Reference))
  (Utilities|IsValid PlayerController
    (:Is%20Valid
      (bind _asbase_player_controller_bp (Utilities|Casting|CastToBasePlayerControllerBP PlayerController)
        (:then
          (CallFunction|ConfirmPlayer _asbase_player_controller_bp player))
        (:CastFailed
          (Development|PrintText "ERROR: LOGIN FAILED" false :!label _label)
          (Game|QuitGame 0 "Quit"))))
    (:Is%20Not%20Valid
      (goto _label))))

(event EventPostPlayerFail
  (params (responseCode :type Integer) (url :type String) (payload :type Va%20Rest%20Json%20Object%20Object%20Reference) (PlayerController :type Player%20Controller%20Object%20Reference))
  (Utilities|ResponseCodeBranch responseCode
    (:404
      _)
    (:500
      _)
    (:-1
      _)
    (:Other
      _))
  (Development|PrintText (Utilities|Text|ToText(String) (Utilities|String|Append "Response code: " (Utilities|String|ToString(Integer) responseCode) " URL: " url " Response: " (Class|VaRestJsonObject|EncodeJsontoSingleString payload)))))

(event EventGetPlayerFail
  (params (responseCode :type Integer) (url :type String) (payload :type Va%20Rest%20Json%20Object%20Object%20Reference) (PlayerController :type Player%20Controller%20Object%20Reference))
  (bind _uniquenetid (Class|AdvancedSessionsLibrary|GetUniqueNetID PlayerController))
  (bind _playername (Class|AdvancedSessionsLibrary|GetPlayerName PlayerController))
  (bind _uniquenetid_2 (Class|AdvancedSessionsLibrary|GetUniqueNetID PlayerController))
  (bind _string (Class|AdvancedSessionsLibrary|UniqueNetIdtoString _uniquenetid))
  (bind _string_2 (Class|AdvancedSessionsLibrary|UniqueNetIdtoString _uniquenetid_2))
  (Utilities|ResponseCodeBranch responseCode
    (:404
      (if (Utilities|Enum|NotEqual(Enum) _string "ERROR, BAD UNIQUE NET ID")
        (Default|PostPlayer (Variables|Default|GetsnowAPI-player) (Utilities|Struct|MakesnowAPI-playerStruct -1 _string _playername "(experience_2_9827AA8747D76E698F4ACE82035899D1=0,base_customization_5_9DDB27CB46D7A8ECC8D264A3FFABFE40=(id_2_257C726C4DDEA1DF509C7FA9E86939A0=0,name_5_A427E6A44A100807C9D0798AB21A95EF=\"starter_base\",slot_8_790168C140BE5C7EB77747A8535601EC=0,drop_odds_10_C2FE72704EDE520A3BF422A8FB0C56B8=0),glove_customization_10_2D6423924911D7239D6FA28D0080CF0C=(id_2_257C726C4DDEA1DF509C7FA9E86939A0=1,name_5_A427E6A44A100807C9D0798AB21A95EF=\"starter_gloves\",slot_8_790168C140BE5C7EB77747A8535601EC=1,drop_odds_10_C2FE72704EDE520A3BF422A8FB0C56B8=0),hat__customization_11_A40669FF4366CAB21B73E39B3ECA92F6=(id_2_257C726C4DDEA1DF509C7FA9E86939A0=2,name_5_A427E6A44A100807C9D0798AB21A95EF=\"starter_hat\",slot_8_790168C140BE5C7EB77747A8535601EC=2,drop_odds_10_C2FE72704EDE520A3BF422A8FB0C56B8=0),eye_customization_12_06788F1D404741583A2ED38DA80F7384=(id_2_257C726C4DDEA1DF509C7FA9E86939A0=3,name_5_A427E6A44A100807C9D0798AB21A95EF=\"starter_eye\",slot_8_790168C140BE5C7EB77747A8535601EC=3,drop_odds_10_C2FE72704EDE520A3BF422A8FB0C56B8=0),chin_customization_14_59B5DEBB49A44DD62429378381A48721=(id_2_257C726C4DDEA1DF509C7FA9E86939A0=4,name_5_A427E6A44A100807C9D0798AB21A95EF=\"starter_chin\",slot_8_790168C140BE5C7EB77747A8535601EC=4,drop_odds_10_C2FE72704EDE520A3BF422A8FB0C56B8=0),color1_19_35FDE41147E36C81CA5554A86A2AC302=(R=1.000000,G=1.000000,B=1.000000,A=0.000000),color2_20_EA06591A450038E68A51CEA2130ADF92=(R=0.000000,G=0.000000,B=0.000000,A=0.000000))") PlayerController)
        (else
          (Default|PostPlayer (Variables|Default|GetsnowAPI-player) (Utilities|Struct|MakesnowAPI-playerStruct -1 _playername _playername "(experience_2_9827AA8747D76E698F4ACE82035899D1=0,base_customization_5_9DDB27CB46D7A8ECC8D264A3FFABFE40=(id_2_257C726C4DDEA1DF509C7FA9E86939A0=0,name_5_A427E6A44A100807C9D0798AB21A95EF=\"starter_base\",slot_8_790168C140BE5C7EB77747A8535601EC=0,drop_odds_10_C2FE72704EDE520A3BF422A8FB0C56B8=0),glove_customization_10_2D6423924911D7239D6FA28D0080CF0C=(id_2_257C726C4DDEA1DF509C7FA9E86939A0=1,name_5_A427E6A44A100807C9D0798AB21A95EF=\"starter_gloves\",slot_8_790168C140BE5C7EB77747A8535601EC=1,drop_odds_10_C2FE72704EDE520A3BF422A8FB0C56B8=0),hat__customization_11_A40669FF4366CAB21B73E39B3ECA92F6=(id_2_257C726C4DDEA1DF509C7FA9E86939A0=2,name_5_A427E6A44A100807C9D0798AB21A95EF=\"starter_hat\",slot_8_790168C140BE5C7EB77747A8535601EC=2,drop_odds_10_C2FE72704EDE520A3BF422A8FB0C56B8=0),eye_customization_12_06788F1D404741583A2ED38DA80F7384=(id_2_257C726C4DDEA1DF509C7FA9E86939A0=3,name_5_A427E6A44A100807C9D0798AB21A95EF=\"starter_eye\",slot_8_790168C140BE5C7EB77747A8535601EC=3,drop_odds_10_C2FE72704EDE520A3BF422A8FB0C56B8=0),chin_customization_14_59B5DEBB49A44DD62429378381A48721=(id_2_257C726C4DDEA1DF509C7FA9E86939A0=4,name_5_A427E6A44A100807C9D0798AB21A95EF=\"starter_chin\",slot_8_790168C140BE5C7EB77747A8535601EC=4,drop_odds_10_C2FE72704EDE520A3BF422A8FB0C56B8=0),color1_19_35FDE41147E36C81CA5554A86A2AC302=(R=1.000000,G=1.000000,B=1.000000,A=0.000000),color2_20_EA06591A450038E68A51CEA2130ADF92=(R=0.000000,G=0.000000,B=0.000000,A=0.000000))") PlayerController))))
    (:500
      (Development|PrintText (Utilities|Text|ToText(String) (Utilities|String|Append "Response code: " (Utilities|String|ToString(Integer) responseCode) " URL: " url " Response: " (Class|VaRestJsonObject|EncodeJsontoSingleString payload))) :!label _label))
    (:-1
      ;[1 1 1] Server is fucked. Go into offline mode
      (bind _asbase_player_controller_bp (Utilities|Casting|CastToBasePlayerControllerBP PlayerController))
      (CallFunction|ConfirmPlayer _asbase_player_controller_bp (Utilities|Struct|MakesnowAPI-playerStruct -1 _string_2 _string_2 "(experience_2_9827AA8747D76E698F4ACE82035899D1=0,base_customization_5_9DDB27CB46D7A8ECC8D264A3FFABFE40=(id_2_257C726C4DDEA1DF509C7FA9E86939A0=0,name_5_A427E6A44A100807C9D0798AB21A95EF=\"starter_base\",slot_8_790168C140BE5C7EB77747A8535601EC=0,drop_odds_10_C2FE72704EDE520A3BF422A8FB0C56B8=0),glove_customization_10_2D6423924911D7239D6FA28D0080CF0C=(id_2_257C726C4DDEA1DF509C7FA9E86939A0=1,name_5_A427E6A44A100807C9D0798AB21A95EF=\"starter_gloves\",slot_8_790168C140BE5C7EB77747A8535601EC=1,drop_odds_10_C2FE72704EDE520A3BF422A8FB0C56B8=0),hat__customization_11_A40669FF4366CAB21B73E39B3ECA92F6=(id_2_257C726C4DDEA1DF509C7FA9E86939A0=2,name_5_A427E6A44A100807C9D0798AB21A95EF=\"starter_hat\",slot_8_790168C140BE5C7EB77747A8535601EC=2,drop_odds_10_C2FE72704EDE520A3BF422A8FB0C56B8=0),eye_customization_12_06788F1D404741583A2ED38DA80F7384=(id_2_257C726C4DDEA1DF509C7FA9E86939A0=3,name_5_A427E6A44A100807C9D0798AB21A95EF=\"starter_eye\",slot_8_790168C140BE5C7EB77747A8535601EC=3,drop_odds_10_C2FE72704EDE520A3BF422A8FB0C56B8=0),chin_customization_14_59B5DEBB49A44DD62429378381A48721=(id_2_257C726C4DDEA1DF509C7FA9E86939A0=4,name_5_A427E6A44A100807C9D0798AB21A95EF=\"starter_chin\",slot_8_790168C140BE5C7EB77747A8535601EC=4,drop_odds_10_C2FE72704EDE520A3BF422A8FB0C56B8=0),color1_19_35FDE41147E36C81CA5554A86A2AC302=(R=1.000000,G=1.000000,B=1.000000,A=0.000000),color2_20_EA06591A450038E68A51CEA2130ADF92=(R=0.000000,G=0.000000,B=0.000000,A=0.000000))")))
    (:Other
      (goto _label))))

(fn ConstructionScript)

(fn ConfirmPlayer
  (params (Controller :type Base%20Player%20Controller%20BP%20Object%20Reference) (apiPlayer :type Snow%20API-player%20Struct%20Structure))
  (LocalVariables|SetincomingApiPlayer apiPlayer)
  (LocalVariables|SetplayerController Controller)
  (bind _assnow_player_state_bp (Utilities|Casting|CastToSnowPlayerStateBP (Variables|/Script/Engine.Controller|GetPlayerState Controller))
    (:then
      (LocalVariables|SetplayerState _assnow_player_state_bp)
      (bind _assnow_game_state_bp (Utilities|Casting|CastToSnowGameStateBP (Game|GetGameState))
        (:then
          (LocalVariables|SetcurrGameState _assnow_game_state_bp)
          (bind _location (CallFunction|GetPlayerSpawnTransform))
          (bind _returnvalue (Game|SpawnActorfromClass "/Game/VRPlayer/VRBaseBP.VRBaseBP_C" _location "AlwaysSpawn" 0 0))
          (bind _output_get (LocalVariables|SetplayerPawn _returnvalue))
          (Pawn|Possess (LocalVariables|GetplayerController) _output_get)
          (Variables|/Game/GameModes/SnowPlayerStateBP.SnowPlayerStateBP_C|SetpawnReference (LocalVariables|GetplayerState) (LocalVariables|GetplayerPawn))
          (Variables|/Game/VRPlayer/VRBaseBP.VRBaseBP_C|SetmyPlayerState (LocalVariables|GetplayerPawn) (LocalVariables|GetplayerState))
          (Default|ClientPostLogin (LocalVariables|GetplayerController))
          (Variables|/Game/GameModes/SnowPlayerStateBP.SnowPlayerStateBP_C|SetapiPlayer (LocalVariables|GetplayerState) (LocalVariables|GetincomingApiPlayer))
          (Default|APIStateChange (LocalVariables|GetplayerPawn))
          (bind _playerscoreindex (Class|SnowGameState|PlayerJoin (LocalVariables|GetcurrGameState) (.steam_id (Utilities|Struct|BreaksnowAPI-playerStruct (LocalVariables|GetincomingApiPlayer)))))
          (Variables|/Script/Snow.SnowPlayerState|SetScoreIndex (LocalVariables|GetplayerState) _playerscoreindex)
          (Variables|Default|SetSpawnOrder (+ (Variables|Default|GetSpawnOrder) 1))
          (Variables|/Game/GameModes/SnowPlayerStateBP.SnowPlayerStateBP_C|SetPlayerColor (LocalVariables|GetplayerState) (Utilities|Array|Get(acopy) (Variables|Default|GetPlayerColors) (Variables|/Script/Snow.SnowPlayerState|GetScoreIndex (LocalVariables|GetplayerState)))))
        (:CastFailed
          (Development|PrintString "Error: Not SnowGameStateBP " false))))
    (:CastFailed
      (Development|PrintString "Error: Not SnowPlayerStateBP " false))))

(fn GetPlayerSpawnTransform
  (bind _outactors (Actor|GetAllActorsOfClass "/Script/Engine.PlayerStart"))
  (return (Math|Transform|MakeTransform (Transformation|GetActorLocation (Utilities|Array|Get(acopy) _outactors (Math|Integer|%(Integer) (Variables|Default|GetSpawnOrder) (Utilities|Array|Length _outactors)))) (Transformation|GetActorRotation (Utilities|Array|Get(acopy) _outactors (Math|Integer|%(Integer) (Variables|Default|GetSpawnOrder) (Utilities|Array|Length _outactors)))))))