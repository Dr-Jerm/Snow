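; SnowGameModeBP is the game mode for a VR snow game, handling player login and spawning.
; On authority, PostLogin queues the controller and requests the player from SnowAPIplayer using a hardcoded "test" Steam ID.
; GetPlayerComplete matches the queued controller, possesses a VRBaseBP spawned at round-robin PlayerStarts, randomizes its customization and registers it with the game state for scoring.
; A failed match quits the game; BeginPlay forces the resolution.
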(event EventPostLogin
  (params (NewPlayer :type Player%20Controller%20Object%20Reference))
  (Networking|SwitchHasAuthority
    (:Authority
      (Default|GetPlayer (Variables|Default|GetsnowAPI-player) -1 "test")
      (Utilities|Array|Add (Variables|Default|GetconnectingPlayers) (Utilities|Struct|MakeConnectingPlayer "test" NewPlayer)))))

(event EventTick
  (params (DeltaSeconds :type Float%20%28single-precision%29)))

(event EventOnSetMatchState
  (params (NewState :type Name)))

(event EventBeginPlay
  (Development|ExecuteConsoleCommand "r.SetRes 2160x1200"))

(event EventGetPlayerComplete
  (params (player :type Snow%20API-player%20Struct%20Structure))
  (bind _playercontroller (CallFunction|GetPlayerfromConnectingPlayers player))
  (Utilities|IsValid _playercontroller
    (:Is%20Valid
      (bind _asbase_player_controller_bp (Utilities|Casting|CastToBasePlayerControllerBP _playercontroller))
      (bind _outactors (Actor|GetAllActorsOfClass "/Script/Engine.PlayerStart"))
      (bind _returnvalue (Game|SpawnActorfromClass "/Game/VRPlayer/VRBaseBP.VRBaseBP_C" (Math|Conversions|ToTransform(Vector) (Transformation|GetActorLocation (Utilities|Array|Get(acopy) _outactors (Math|Integer|%(Integer) (Variables|Default|GetSpawnOrder) (Utilities|Array|Length _outactors))))) "AlwaysSpawn" 0 0))
      (Pawn|Possess _asbase_player_controller_bp _returnvalue)
      (Default|ClientPostLogin _asbase_player_controller_bp)
      (Variables|/Script/Snow.VRBase|SetCustomization _returnvalue (Utilities|Array|MakeArray (Math|Integer|%(Integer) (Math|Random|RandomInteger 10) 2) (Math|Integer|%(Integer) (Math|Random|RandomInteger 10) 2) (Math|Integer|%(Integer) (Math|Random|RandomInteger 10) 2) (Math|Integer|%(Integer) (Math|Random|RandomInteger 10) 2) (Math|Integer|%(Integer) (Math|Random|RandomInteger 10) 2)))
      (Default|VisualChange _returnvalue)
      (bind _assnow_game_state_bp (Utilities|Casting|CastToSnowGameStateBP (Game|GetGameState)))
      (bind _assnow_player_state_bp (Utilities|Casting|CastToSnowPlayerStateBP (Variables|/Script/Engine.Controller|GetPlayerState _asbase_player_controller_bp)))
      (bind _playerscoreindex (Class|SnowGameState|PlayerJoin _assnow_game_state_bp (Variables|/Script/Engine.PlayerState|GetPlayerId _assnow_player_state_bp)))
      (Variables|/Script/Snow.SnowPlayerState|SetScoreIndex _assnow_player_state_bp _playerscoreindex)
      (Variables|Default|SetSpawnOrder (+ (Variables|Default|GetSpawnOrder) 1))
      (Variables|/Game/VRPlayer/SnowPlayerStateBP.SnowPlayerStateBP_C|SetpawnReference _assnow_player_state_bp _returnvalue))
    (:Is%20Not%20Valid
      (Development|PrintText "ERROR: LOGIN FAILED" false)
      (Game|QuitGame 0 "Quit"))))

(fn ConstructionScript)

(fn GetPlayerfromConnectingPlayers
  (params (PlayerStruct :type Snow%20API-player%20Struct%20Structure))
  (bind (_array_element _array_index) (Utilities|Array|ForEachLoopwithBreak (Variables|Default|GetconnectingPlayers))
    (:LoopBody
      (if (Utilities|Enum|Equal(Enum) (.id (Utilities|Struct|BreakConnectingPlayer _array_element)) (.steam_id (Utilities|Struct|BreaksnowAPI-playerStruct PlayerStruct)))
        (LocalVariables|SetPC (.playerController (Utilities|Struct|BreakConnectingPlayer _array_element)))
        (Utilities|Array|RemoveIndex (Variables|Default|GetconnectingPlayers) _array_index)
        (return (LocalVariables|GetPC))))
    (:Completed
      (return 0))))