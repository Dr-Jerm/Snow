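; HordeGameStateBP is the game state for the horde game mode and drives horde progression through a state machine.
; On BeginPlay it spawns a WaitHordeState actor as the initial state.
; Each tick it executes the current state; once that reports completion, it takes the next state from it, destroys the finished actor and switches over.
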(event EventBeginPlay
  (|CallParentFunction)
  (bind _returnvalue (Game|SpawnActorfromClass "/Game/Events/HordeEvents/WaitHordeState.WaitHordeState_C" (Math|Transform|MakeTransform "0, 0, 0") "Undefined" 0 0))
  (Variables|Default|SetHordeState _returnvalue))

(event EventTick
  (params (DeltaSeconds :type Float%20%28single-precision%29))
  (|CallParentFunction DeltaSeconds)
  (Default|Execute (Variables|Default|GetHordeState))
  (if (Variables|/Game/Events/HordeEvents/HordeState.HordeState_C|GetIsComplete (Variables|Default|GetHordeState))
    (bind _hordestate (Default|GetNextState (Variables|Default|GetHordeState)))
    (Actor|DestroyActor (Variables|Default|GetHordeState))
    (Variables|Default|SetHordeState _hordestate)))

(fn ConstructionScript
  (|CallParentFunction))