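; HordeGameModeBP is the Blueprint game mode for the Horde mode, acting as a thin child of a parent class that holds any actual behavior.
; Its tick, begin play, login, logout, server restart and restart broadcast events only forward to the parent implementations.
; The construction script likewise calls only its parent, so the graphs shown add no logic of their own.
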(event EventBeginPlay
  (|CallParentFunction))

(event EventServerRestart
  (|CallParentFunction))

(event EventPostLogin
  (params (NewPlayer :type Player%20Controller%20Object%20Reference))
  (|CallParentFunction NewPlayer))

(event EventBroadcastRestart
  (|CallParentFunction))

(event EventOnLogout
  (params (ExitingController :type Controller%20Object%20Reference))
  (|CallParentFunction ExitingController))

(event EventTick
  (params (DeltaSeconds :type Float%20%28single-precision%29))
  (|CallParentFunction DeltaSeconds))

(fn ConstructionScript
  (|CallParentFunction))