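; Player state Blueprint for the Horde game mode that defines how a player's score is reported.
; GetScore reads a single score item, selected by an enum entry, and truncates it to an integer.
; Tick, knockout and damage events only forward to the parent class, while BeginPlay and ChangeState are empty.
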(event EventBeginPlay)

(event EventTick
  (params (DeltaSeconds :type Float%20%28single-precision%29))
  (|CallParentFunction DeltaSeconds))

(event EventTakeDamage
  (params (Damage :type Float%20%28single-precision%29) (HitDirection :type Vector) (InstigatedBy :type Controller%20Object%20Reference) (DamageCauser :type Actor%20Object%20Reference))
  (|CallParentFunction Damage HitDirection InstigatedBy DamageCauser))

(event EventBeKnockedOut
  (params (Source :type Controller%20Object%20Reference) (DamageCauser :type Actor%20Object%20Reference))
  (|CallParentFunction Source DamageCauser))

(fn ConstructionScript
  (|CallParentFunction))

(fn ChangeState)

(fn GetScore
  (bind _score (CallFunction|GetScoreItem "NewEnumerator7"))
  (return (Math|Float|Truncate _score)))