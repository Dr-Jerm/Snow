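; Game state for the Brawl game mode that handles end-of-round timing and audio cues.
; On authority, Tick compares server world time against the start wait and game lengths to fire one-shot closing music and final countdown ticking, each guarded by a flag.
; Once the end wait also elapses, it calls LeaveSession on the Steam game instance.
; The GameEnd event is an empty stub.
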(event EventBeginPlay)

(event EventTick
  (params (DeltaSeconds :type Float%20%28single-precision%29))
  (|CallParentFunction DeltaSeconds)
  (Networking|SwitchHasAuthority
    (:Authority
      (Utilities|FlowControl|Sequence
        (:then_0
          (if (and (> (GameState|GetServerWorldTimeSeconds (Game|GetGameState)) (- (+ (Variables|SetByGameMode|GetStartWaitLength) (Variables|SetByGameMode|GetGameLength)) 54.0)) (not (Variables|Default|GetisEndMusicPlaying)))
            (Variables|Default|SetisEndMusicPlaying true)
            (CallFunction|PlayEndgameMusic)))
        (:then_1
          (if (and (> (GameState|GetServerWorldTimeSeconds (Game|GetGameState)) (- (+ (Variables|SetByGameMode|GetStartWaitLength) (Variables|SetByGameMode|GetGameLength)) 6.8)) (not (Variables|Default|GetisTenSecondsLeft)))
            (Variables|Default|SetisTenSecondsLeft true)
            (CallFunction|10SecondsLeft)))
        (:then_2
          (if (> (GameState|GetServerWorldTimeSeconds (Game|GetGameState)) (+ (Variables|SetByGameMode|GetStartWaitLength) (Variables|SetByGameMode|GetGameLength) (Variables|SetByGameMode|GetEndWaitLength)))
            (bind _assteam_game_instance_bp (Utilities|Casting|CastToSteamGameInstanceBP (Game|GetGameInstance)))
            (Default|LeaveSession _assteam_game_instance_bp "None")))))))

(event Custom|PlayEndgameMusic
  (Audio|PlaySound2D "/Game/Assets/sound/RoundEvents/roundEnd_52s.roundEnd_52s" 0.5))

(event Custom|GameEnd)

(event Custom|10SecondsLeft
  (Audio|PlaySound2D "/Game/Assets/sound/10_sec_tick.10_sec_tick" 0.2))

(fn ConstructionScript)