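; BrawlPlayerStateBP is the player state for the Brawl game mode, tracking player health and its automatic regeneration.
; Health starts at the base value in the construction script.
; On the server, Tick accumulates time since last damage and, after a wait period, refills health at a linear rate set by the total regen time, capped at base health.
; The pawn broadcasts when regeneration begins and ends.
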(event EventBeginPlay)

(event EventTick
  (params (DeltaSeconds :type Float%20%28single-precision%29))
  (Networking|SwitchHasAuthority
    (:Authority
      (Utilities|FlowControl|Sequence
        (:then_0
          (CallFunction|ProcessHealthRegen DeltaSeconds))))))

(fn ConstructionScript
  (Variables|Health|SetCurrentHealth (Variables|Health|GetBaseHealth)))

(fn ProcessHealthRegen
  (params (delta :type Float%20%28single-precision%29))
  (bind _output_get (LocalVariables|SettmpDelta delta))
  (Variables|Default|SettimeSinceLastDamage (+ _output_get (Variables|Default|GettimeSinceLastDamage)))
  (if (and (>= (Variables|Default|GettimeSinceLastDamage) (Variables|Health|GetBaseHealthRegenWaitTime)) (< (Variables|Health|GetCurrentHealth) (Variables|Health|GetBaseHealth)))
    (if (Variables|Default|GetisRegeneratingHealth)
      _
      (else
        (Variables|Default|SetisRegeneratingHealth true)
        (Default|BroadcastBeginHealthRegen (Variables|Default|GetpawnReference))))
    (bind _output_get_2 (LocalVariables|SetammountToIncrementHealth (/ (Variables|Health|GetBaseHealth) (/ (Variables|Health|GetBaseHealthRegenTime) (LocalVariables|GettmpDelta)))))
    (Variables|Health|SetCurrentHealth (Math|Float|Min(Float) (Variables|Health|GetBaseHealth) (+ _output_get_2 (Variables|Health|GetCurrentHealth))))
    (elif (Variables|Default|GetisRegeneratingHealth)
      (Variables|Default|SetisRegeneratingHealth false)
      (Default|BroadcastEndHealthRegen (Variables|Default|GetpawnReference)))))