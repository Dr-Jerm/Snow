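; Game mode for health-based VR snowball play, where head hits from players or AI snowmen damage the target's HealthPlayerStateBP.
; Hit and input overrides gate actions, with Invisible and Ghost players immune to head damage and blocked from trigger use.
; Players spawn at the first SpawnBox, matches are always ready to start and end on IsEndGame.
; It also provides a restart broadcast and JSON round start/end logging through Logger.
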(event EventPostLogin
  (params (NewPlayer :type Player%20Controller%20Object%20Reference))
  (|CallParentFunction NewPlayer))

(event EventOnLogout
  (params (ExitingController :type Controller%20Object%20Reference))
  (|CallParentFunction ExitingController))

(event EventBeginPlay
  (|CallParentFunction))

(event Custom|BroadcastRestart
  (Class|GameMode|RestartGame))

(event Custom|ServerRestart
  (CallFunction|BroadcastRestart))

(fn ConstructionScript)

(fn ReadytoEndMatch
  (return (Variables|Default|GetisEndGame)))

(fn BuildLog
  (params (roundStart :type Boolean) (numberOfPlayers :type Integer) (totalScore :type Integer))
  (bind _roundlogdata (Utilities|Struct|MakeRoundLogData numberOfPlayers roundStart totalScore))
  (bind (_numberofplayers _start _totalscore) (Utilities|Struct|BreakRoundLogData _roundlogdata))
  (LocalVariables|SetjsonObj (Class|VaRestJsonObject|ConstructJsonObject))
  (Class|VaRestJsonObject|SetNumberField (LocalVariables|GetjsonObj) "numberOfPlayers" (Math|Conversions|ToFloat(Integer) _numberofplayers))
  (Class|VaRestJsonObject|SetBoolField (LocalVariables|GetjsonObj) "isStart" _start)
  (Class|VaRestJsonObject|SetNumberField (LocalVariables|GetjsonObj) "totalScore" (Math|Conversions|ToFloat(Integer) _totalscore))
  (return (LocalVariables|GetjsonObj)))

(fn RoundStartEndLog
  (params (TotalKnockouts :type Integer) (PlayerCount :type Integer) (isStart :type Boolean))
  (LocalVariables|SetplayerCountTmp PlayerCount)
  (bind _json (Logging|BuildLog isStart (LocalVariables|GetplayerCountTmp) TotalKnockouts))
  (Default|SubmitLog (Variables|Default|GetLogger) _json self))

(fn ReadytoStartMatch
  (return true))

(fn GetPlayerSpawnTransform
  (bind _outactors (Actor|GetAllActorsOfClass "/Game/Blueprints/SpawnBox.SpawnBox_C"))
  (if (> (Utilities|Array|Length _outactors) 0)
    (return (Math|Transform|MakeTransform (Transformation|GetWorldLocation (Variables|/Game/Blueprints/SpawnBox.SpawnBox_C|GetDefaultSceneRoot (Utilities|Array|Get(acopy) _outactors))) "0, 0, 0" "1.000000,1,1"))
    (else
      (bind _location (|CallParentFunction))
      (return _location))))

(fn HeadHitOverride
  (params (Hit :type Hit%20Result%20Structure) (Snowball :type A%20Snowball%20Replicated%20Object%20Reference) (HitPawn :type VR%20Base%20BP%20Object%20Reference))
  (LocalVariables|SetHitRef Hit)
  (LocalVariables|SetSnowballRef Snowball)
  (bind _output_get (LocalVariables|SetTargetPlayerPawn HitPawn))
  (bind _ashealth_player_state_bp (Utilities|Casting|CastToHealthPlayerStateBP (Variables|/Game/VRPlayer/VRBaseBP.VRBaseBP_C|GetmyPlayerState _output_get))
    (:then
      (bind _output_get_2 (LocalVariables|SetTargetHealthPlayerState _ashealth_player_state_bp))
      (switch Utilities|FlowControl|Switch|SwitchonBrawlPlayerModes (Variables|/Game/GameModes/HealthGameMode/HealthPlayerStateBP.HealthPlayerStateBP_C|GetplayerMode _output_get_2)
        (:NewEnumerator0
          _)
        (:NewEnumerator1
          _)
        (:NewEnumerator2
          (bind _asvrbase_bp (Utilities|Casting|CastToVRBaseBP (Components|GetOwner (LocalVariables|GetSnowballRef)) :!label _label)
            (:then
              (LocalVariables|SetSourcePlayerPawn _asvrbase_bp)
              (Default|TakeDamage (LocalVariables|GetTargetHealthPlayerState) (Variables|/Game/Assets/Snowball/ASnowball_replicated.ASnowball_replicated_C|Getdamage (LocalVariables|GetSnowballRef)) (Math|Vector|NegateVector (.Normal (Collision|BreakHitResult (LocalVariables|GetHitRef)))) (Pawn|GetController (LocalVariables|GetSourcePlayerPawn)) (LocalVariables|GetSnowballRef))
              (return true))
            (:CastFailed
              (bind _asai_snowman_basic (Utilities|Casting|CastToAI_SnowmanBasic (Components|GetOwner (LocalVariables|GetSnowballRef)))
                (:then
                  (bind _ashealth_player_state_bp_2 (Utilities|Casting|CastToHealthPlayerStateBP (Variables|/Game/VRPlayer/VRBaseBP.VRBaseBP_C|GetmyPlayerState (LocalVariables|GetTargetPlayerPawn)))
                    (:then
                      (Default|TakeDamage _ashealth_player_state_bp_2 (Variables|/Game/Assets/Snowball/ASnowball_replicated.ASnowball_replicated_C|Getdamage (LocalVariables|GetSnowballRef)) (Math|Vector|NegateVector (.Normal (Collision|BreakHitResult (LocalVariables|GetHitRef)))) (Pawn|GetController _asai_snowman_basic) (LocalVariables|GetSnowballRef))
                      (return true))
                    (:CastFailed
                      (return true))))
                (:CastFailed
                  (return false))))))
        (:NewEnumerator3
          (goto _label)))
      (return false))
    (:CastFailed
      (return false))))

(fn MittenHitOverride
  (params (Hit :type Hit%20Result%20Structure) (Snowball :type A%20Snowball%20Replicated%20Object%20Reference) (HitPawn :type VR%20Base%20BP%20Object%20Reference))
  (return true))

(fn TeleportOverride
  (params (TeleportLocation :type Vector :default "0, 0, 0"))
  (return true))

(fn ThumbpadOverride
  (params (ThumbpadComponent :type Thumbpad%20Component%20Object%20Reference) (Pressed :type Boolean) (Hand :type EControllerHand%20Enum :default "Left"))
  (return true))

(fn TriggerOverride
  (params (Pressed :type Boolean) (Hand :type EControllerHand%20Enum :default "Left") (TriggerComponent :type Trigger%20Component%20Object%20Reference))
  (bind _asvrbase_bp (Utilities|Casting|CastToVRBaseBP (Components|GetOwner TriggerComponent))
    (:then
      (bind _ashealth_player_state_bp (Utilities|Casting|CastToHealthPlayerStateBP (Variables|/Game/VRPlayer/VRBaseBP.VRBaseBP_C|GetmyPlayerState _asvrbase_bp))
        (:then
          (switch Utilities|FlowControl|Switch|SwitchonBrawlPlayerModes (Variables|/Game/GameModes/HealthGameMode/HealthPlayerStateBP.HealthPlayerStateBP_C|GetplayerMode _ashealth_player_state_bp)
            (:NewEnumerator0
              _)
            (:NewEnumerator1
              _)
            (:NewEnumerator2
              (return true))
            (:NewEnumerator3
              (return true))))
        (:CastFailed
          (return true))))
    (:CastFailed
      _))
  (return false))