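; Player state for the health game mode in a VR snowball fight, tracking health, player mode and score.
; Authority-only Tick regenerates health after a damage-free delay and runs Ghost and Invisible timers, teleporting to a random PlayerStart between them.
; TakeDamage only hurts Standard players, credits the attacker's score and triggers knockout, broadcasting changes through the pawn.
; Score modifiers are fetched but unapplied; scores print for debugging.
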(event Custom|OnWaitingPostMatch)

(event EventBeginPlay
  (|CallParentFunction))

(event EventTick
  (params (DeltaSeconds :type Float%20%28single-precision%29))
  (|CallParentFunction DeltaSeconds)
  (Networking|SwitchHasAuthority
    (:Authority
      (Utilities|FlowControl|Sequence
        (:then_0
          (CallFunction|ProcessHealthRegen DeltaSeconds))
        (:then_1
          (CallFunction|ProcessPlayerModesandRespawn DeltaSeconds))
        (:then_2
          (for _array_element (Variables|Default|GetScoreItems)
            (if (!= (.Score (Utilities|Struct|BreakScoreItem _array_element)) 0.0)
              (Development|PrintString (Utilities|String|Append (Utilities|String|EnumtoString (.ScoreType (Utilities|Struct|BreakScoreItem _array_element))) ": " (Utilities|String|ToString(Float) (.Score (Utilities|Struct|BreakScoreItem _array_element))))))))))))

(event EventReset
  (|CallParentFunction)
  (Variables|PlayerMode|SetplayerMode "NewEnumerator2"))

(fn ConstructionScript
  (Variables|Health|SetCurrentHealth (Variables|Health|GetBaseHealth)))

(fn ProcessHealthRegen
  (params (delta :type Float%20%28single-precision%29))
  (bind _output_get (LocalVariables|SettmpDelta delta))
  (Variables|Health|SettimeSinceLastDamage (+ _output_get (Variables|Health|GettimeSinceLastDamage)))
  (if (and (>= (Variables|Health|GettimeSinceLastDamage) (Variables|Health|GetBaseHealthRegenWaitTime)) (< (Variables|Health|GetCurrentHealth) (Variables|Health|GetBaseHealth))) ; Been enough time and not max
    (if (Variables|Health|GetisRegeneratingHealth) ; Already been regenerating?
      _
      (else
        (Variables|Health|SetisRegeneratingHealth true)
        (Default|BroadcastBeginHealthRegen (Variables|Default|GetpawnReference))))
    (bind _output_get_2 (LocalVariables|SetamountToIncrementHealth (/ (Variables|Health|GetBaseHealth) (/ (Variables|Health|GetBaseHealthRegenTime) (LocalVariables|GettmpDelta)))))
    (Variables|Health|SetCurrentHealth (Math|Float|Min(Float) (Variables|Health|GetBaseHealth) (+ _output_get_2 (Variables|Health|GetCurrentHealth))))
    (elif (Variables|Health|GetisRegeneratingHealth) ; First time stopping?
      (Variables|Health|SetisRegeneratingHealth false)
      (Default|BroadcastEndHealthRegen (Variables|Default|GetpawnReference)))))

(fn OnRepPlayerMode
  (switch Utilities|FlowControl|Switch|SwitchonBrawlPlayerModes (Variables|PlayerMode|GetplayerMode)))

(fn ReduceHealth
  (params (Damage :type Float%20%28single-precision%29))
  (Variables|Health|SetCurrentHealth (- (Variables|Health|GetCurrentHealth) Damage))
  (Variables|Health|SettimeSinceLastDamage 0.0)
  (return))

(fn BeKnockedOut
  (params (Source :type Controller%20Object%20Reference) (DamageCauser :type Actor%20Object%20Reference))
  (LocalVariables|SetKnockoutSourceActor DamageCauser)
  (bind _asbase_player_controller_bp (Utilities|Casting|CastToBasePlayerControllerBP Source)
    (:then
      (bind _output_get (LocalVariables|SetKnockoutPlayerController _asbase_player_controller_bp))
      (bind _asvrbase_bp (Utilities|Casting|CastToVRBaseBP (Pawn|GetControlledPawn _output_get)))
      (LocalVariables|SetKnockoutPawn _asvrbase_bp)
      (bind _ashealth_player_state_bp (Utilities|Casting|CastToHealthPlayerStateBP (Variables|/Script/Engine.Controller|GetPlayerState (LocalVariables|GetKnockoutPlayerController))))
      (if (!= _ashealth_player_state_bp self)
        _
        (else
          _)))
    (:CastFailed
      _))
  (bind _asasnowball_replicated (Utilities|Casting|CastToASnowball_replicated (LocalVariables|GetKnockoutSourceActor)))
  (bind _returnvalue (Physics|GetPhysicsLinearVelocity (Variables|/Game/Assets/Snowball/ASnowball_replicated.ASnowball_replicated_C|GetSphere_0 _asasnowball_replicated) "None"))
  (Variables|PlayerMode|SetplayerMode "NewEnumerator1")
  (Variables|PlayerMode|SetRemainingGhostTime (Variables|PlayerMode|GetBaseGhostTime))
  (Variables|PlayerMode|SetRemainingInvisibilityTime (Variables|PlayerMode|GetBaseInvisibilityTime))
  (Variables|Health|SetCurrentHealth (Variables|Health|GetBaseHealth))
  (Default|BroadcastGoGhost (Variables|Default|GetpawnReference) (GameState|GetServerWorldTimeSeconds (Game|GetGameState)) _returnvalue))

(fn TakeDamage
  (params (Damage :type Float%20%28single-precision%29) (HitDirection :type Vector) (InstigatedBy :type Controller%20Object%20Reference) (DamageCauser :type Actor%20Object%20Reference))
  (bind _currenthealth (Variables|Health|GetCurrentHealth))
  (bind _returnvalue (<= _currenthealth 0.0))
  (Utilities|FlowControl|Sequence
    (:then_0
      (LocalVariables|SetdamageRef Damage))
    (:then_1
      (LocalVariables|SetHitNormalRef HitDirection))
    (:then_2
      (LocalVariables|SetInstigatedByRef InstigatedBy))
    (:then_3
      (LocalVariables|SetDamageCauserRef DamageCauser))
    (:then_4
      (Utilities|FlowControl|Sequence
        (:then_0
          (bind _asbase_player_controller_bp (Utilities|Casting|CastToBasePlayerControllerBP (LocalVariables|GetInstigatedByRef)))
          (Default|PlaySound _asbase_player_controller_bp "/Game/Assets/sound/Scoring/Enemy_SBHitV1.Enemy_SBHitV1") ; Thrower gets successfulHitSound
        )
        (:then_1
          (if (Utilities|Enum|Equal(Enum) (Variables|PlayerMode|GetplayerMode) "NewEnumerator2") ; Can be hit/scored?
            (CallFunction|ReduceHealth (LocalVariables|GetdamageRef))
            (bind _ashealth_player_state_bp (Utilities|Casting|CastToHealthPlayerStateBP (Variables|/Script/Engine.Controller|GetPlayerState (LocalVariables|GetInstigatedByRef)))
              (:then
                (if _returnvalue ; Has Lethal Damage?
                  (CallFunction|ScorePoint _ashealth_player_state_bp "NewEnumerator4" self (LocalVariables|GetdamageRef))
                  (else
                    (CallFunction|ScorePoint _ashealth_player_state_bp "NewEnumerator0" self (LocalVariables|GetdamageRef))
                    (return))))
              (:CastFailed
                (if _returnvalue
                  _
                  (else
                    (return)))))
            (CallFunction|BeKnockedOut (LocalVariables|GetInstigatedByRef) (LocalVariables|GetDamageCauserRef))
            (return)
            (else
              (return))))))))

(fn ProcessPlayerModesandRespawn
  (params (delta :type Float%20%28single-precision%29))
  (switch Utilities|FlowControl|Switch|SwitchonBrawlPlayerModes (Variables|PlayerMode|GetplayerMode)
    (:NewEnumerator0
      (bind _output_get (Variables|PlayerMode|SetRemainingInvisibilityTime (- (Variables|PlayerMode|GetRemainingInvisibilityTime) delta)))
      (if (<= _output_get 0.0)
        (Variables|PlayerMode|SetplayerMode "NewEnumerator2")
        (Default|BroadcastRespawn (Variables|Default|GetpawnReference))))
    (:NewEnumerator1
      (bind _output_get_2 (Variables|PlayerMode|SetRemainingGhostTime (- (Variables|PlayerMode|GetRemainingGhostTime) delta)))
      (if (<= _output_get_2 0.0)
        (Variables|PlayerMode|SetplayerMode "NewEnumerator0")
        (Default|BroadcastGoInvisible (Variables|Default|GetpawnReference))
        (bind _outactors (Actor|GetAllActorsOfClass "/Script/Engine.PlayerStart"))
        (CallFunction|TeleporttoActor (Variables|Default|GetpawnReference) (Utilities|Array|Get(acopy) _outactors (Math|Random|RandomIntegerinRange 0 (- (Utilities|Array|Length _outactors) 1))))))))

(fn ValidTarget
  (bind _playermode (Variables|PlayerMode|GetplayerMode))
  (bind _valid (|CallParentFunction))
  (return (and _valid (or (Utilities|Enum|Equal(Enum) _playermode "NewEnumerator2") (Utilities|Enum|Equal(Enum) _playermode "NewEnumerator3")))))

(fn ScorePoint
  (params (ScoreType :type ScoreTypeEnum%20Enum) (TargetPlayer :type Health%20Player%20State%20BP%20Object%20Reference) (ScoreInput :type Float%20%28single-precision%29))
  (LocalVariables|SetLocalScoreType ScoreType)
  (LocalVariables|SetLocalScoreInput ScoreInput)
  (bind _scoremodifiers (CallFunction|GetScoreModifiers))
  (for _array_element _scoremodifiers
    (switch Utilities|FlowControl|Switch|SwitchonScoreModifierEnum (.ModifierType (Utilities|Struct|BreakScoreModifier _array_element))))
  (CallFunction|AssignScoretoType (LocalVariables|GetLocalScoreInput) (LocalVariables|GetLocalScoreType))
  (Development|PrintString (Utilities|String|ToString(Float) (LocalVariables|GetLocalScoreInput))))

(fn GetScoreModifiers
  (bind _ashealth_game_state_bp (Utilities|Casting|CastToHealthGameStateBP (Game|GetGameState))
    (:then
      (for _array_element (Variables|/Game/GameModes/HealthGameMode/HealthGameStateBP.HealthGameStateBP_C|GetScoreModifiers _ashealth_game_state_bp)
        (if (== (.Receiver (Utilities|Struct|BreakScoreModifier _array_element)) self)
          (Utilities|Array|Add (LocalVariables|GetReturnedScoreModifiers) _array_element)))
      (return (LocalVariables|GetReturnedScoreModifiers)))
    (:CastFailed
      (return (LocalVariables|GetReturnedScoreModifiers)))))

(fn AssignScoretoType
  (params (Score :type Float%20%28single-precision%29) (ScoreType :type ScoreTypeEnum%20Enum))
  (for (_array_element _array_index) (Variables|Default|GetScoreItems)
    (if (Utilities|Enum|Equal(Enum) ScoreType (.ScoreType (Utilities|Struct|BreakScoreItem _array_element)))
      (Utilities|Array|SetArrayElem (Variables|Default|GetScoreItems) _array_index (Utilities|Struct|MakeScoreItem (.ScoreType (Utilities|Struct|BreakScoreItem _array_element)) (+ (.Score (Utilities|Struct|BreakScoreItem _array_element)) Score))))))

(fn GetHealth
  (return (Variables|Health|GetBaseHealth) (Variables|Health|GetCurrentHealth)))