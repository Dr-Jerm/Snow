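; Game mode for Snow Day's VR tutorial, with timed or action-gated steps for walking, teleporting, trigger use, and grabbing and throwing snow.
; Each Teach function sets pawn help text, highlights or hand visuals, advancing through ChangeTutorialState.
; The state dispatch and per-state input gating are disconnected: Tick only updates timers and a flag, and overrides return constants.
; Player confirmation still enables noob hands after a short delay for material setup.
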(event Custom|ChangeTutorialState
  (params (TutState :type TutorialStateEnum%20Enum))
  (Variables|Default|SetPreviousLocation (Transformation|GetWorldLocation (Variables|/Game/VRPlayer/VRBaseBP.VRBaseBP_C|GetHeadCollisionVolume (Variables|Default|GetPlayerPawn_0))))
  (Variables|Default|SetCurrentStateTime 0.0)
  (Variables|Default|SetTutorialState TutState)
  (Variables|Default|SetTriggerTimesPulled 0))

(event EventTick
  (params (DeltaSeconds :type Float%20%28single-precision%29))
  (Variables|Default|SetDeltaTime DeltaSeconds)
  (Variables|Default|SetCurrentStateTime (+ (Variables|Default|GetDeltaTime) (Variables|Default|GetCurrentStateTime)))
  (Variables|Default|SetThumbpadPush false))

(event EventConfirmPlayer
  (params (Controller :type Base%20Player%20Controller%20BP%20Object%20Reference) (apiPlayer :type Snow%20API-player%20Struct%20Structure))
  (|CallParentFunction Controller apiPlayer)
  (Utilities|FlowControl|Delay 0.1) ; Something sets the left hand materials,\nso need to wait for that to resolve before \ngoing into noob mode
  (CallFunction|TutorialPawnSetup Controller))

(fn ConstructionScript)

(fn TeachWalkAround
  (params (DeltaTime :type Float%20%28single-precision%29))
  (bind _playerpawn_0 (Variables|Default|GetPlayerPawn_0))
  (bind _headcollisionvolume (Variables|/Game/VRPlayer/VRBaseBP.VRBaseBP_C|GetHeadCollisionVolume _playerpawn_0))
  (bind _returnvalue (Transformation|GetWorldLocation _headcollisionvolume))
  (Utilities|FlowControl|Sequence
    (:then_0
      (if (> (Math|Vector|VectorLength (- (Variables|Default|GetPreviousLocation) _returnvalue)) 0.1)
        (Variables|Default|SetTotalDistanceTraveled (+ (Math|Vector|VectorLength (- (Variables|Default|GetPreviousLocation) _returnvalue)) (Variables|Default|GetTotalDistanceTraveled)))
        (Variables|Default|SetPreviousLocation _returnvalue)))
    (:then_1
      (if (< (Variables|Default|GetTotalDistanceTraveled) 2.5e+02)
        (bind _output_get (LocalVariables|SetPlayerText "Welcome to Snow Day! Here are the 
basics you'll need to play. We'll start 
by walking around. Simply  
walk around as you would in real life.  
If you see a grid appear, you've gone 
too far! Go ahead and try walking within 
the grid."))
        (Rendering|Components|TextRender|SetText (Variables|/Game/VRPlayer/VRBaseBP.VRBaseBP_C|GetHelpText (Variables|Default|GetPlayerPawn_0)) (Utilities|Text|ToText(String) _output_get))
        (elif (< (Variables|Default|GetTotalDistanceTraveled) 5e+02)
          (bind _output_get_2 (LocalVariables|SetPlayerText "Keep going! You're almost there! 
Remember you can also turn your 
body to look around."))
          (Rendering|Components|TextRender|SetText (Variables|/Game/VRPlayer/VRBaseBP.VRBaseBP_C|GetHelpText (Variables|Default|GetPlayerPawn_0)) (Utilities|Text|ToText(String) _output_get_2))
          (else
            (CallFunction|ChangeTutorialState "NewEnumerator5")))))))

(fn TeachPullTrigger
  (params (DeltaTime :type Float%20%28single-precision%29))
  (bind _playerpawn_0 (Variables|Default|GetPlayerPawn_0))
  (bind _triggercomponent (Variables|/Game/VRPlayer/VRBaseBP.VRBaseBP_C|GetTriggerComponent _playerpawn_0))
  (bind _output_get (LocalVariables|SetPlayerText "Turn your controllers over. You'll see 
two buttons highlighted in yellow. 
Use your forefinger to give each 
of them a few squeezes."))
  (Default|HighlightTrigger _triggercomponent "Left" true)
  (Default|HighlightTrigger _triggercomponent "Right" true)
  (Rendering|Components|TextRender|SetText (Variables|/Game/VRPlayer/VRBaseBP.VRBaseBP_C|GetHelpText (Variables|Default|GetPlayerPawn_0)) (Utilities|Text|ToText(String) _output_get))
  (CallFunction|ChangeTutorialState "NewEnumerator8"))

(fn TeachThrowSnow
  (params (DeltaTime :type Float%20%28single-precision%29))
  (if (Variables|Default|GetHasThrown)
    (if (Variables|Default|GetSuccessfulThrow)
      (CallFunction|ChangeTutorialState "NewEnumerator6")
      (else
        (bind _output_get (LocalVariables|SetHelpText "Nice try, but you'll need to try throwing 
harder than that if you expect to hit 
anybody. Pick up another snowball 
and try again."))
        (Rendering|Components|TextRender|SetText (Variables|/Game/VRPlayer/VRBaseBP.VRBaseBP_C|GetHelpText (Variables|Default|GetPlayerPawn_0)) (Utilities|Text|ToText(String) _output_get))))
    (else
      (bind _output_get_2 (LocalVariables|SetHelpText "Radical! Now, make a throwing motion and 
let go of the snowball. "))
      (Rendering|Components|TextRender|SetText (Variables|/Game/VRPlayer/VRBaseBP.VRBaseBP_C|GetHelpText (Variables|Default|GetPlayerPawn_0)) (Utilities|Text|ToText(String) _output_get_2)))))

(fn TeachTeleport
  (params (DeltaTime :type Float%20%28single-precision%29))
  (bind _playerpawn_0 (Variables|Default|GetPlayerPawn_0))
  (bind _thumbpadcomponent (Variables|/Game/VRPlayer/VRBaseBP.VRBaseBP_C|GetThumbpadComponent _playerpawn_0))
  (if (< (Variables|Default|GetCurrentStateTime) 1.0)
    (bind _output_get (LocalVariables|SetTeleportString "Take a look at your controller.  
You'll see a big round button  
that's highlighted in yellow. 
Press and release it to teleport."))
    (Rendering|Components|TextRender|SetText (Variables|/Game/VRPlayer/VRBaseBP.VRBaseBP_C|GetHelpText _playerpawn_0) (Utilities|Text|ToText(String) _output_get))
    (Default|HighlightThumbpad _thumbpadcomponent "Left" true)
    (Default|HighlightThumbpad _thumbpadcomponent "Right" true)
    (else
      (Variables|Default|SetThumbpadPush true)
      (if (Variables|Default|GetAllowTeleport)
        (Default|HighlightThumbpad _thumbpadcomponent "Left" false)
        (Default|HighlightThumbpad _thumbpadcomponent "Right" false)
        (CallFunction|ChangeTutorialState "NewEnumerator10")))))

(fn TeachDone
  (params (DeltaTime :type Float%20%28single-precision%29))
  (Rendering|Components|TextRender|SetText (Variables|/Game/VRPlayer/VRBaseBP.VRBaseBP_C|GetHelpText (Variables|Default|GetPlayerPawn_0)) (Utilities|Text|ToText(String) "Great job! You're ready for a real snow 
brawl. To return to your bedroom, grab 
the doorknob on the house.")))

(fn TeachWelcome
  (params (DeltaTime :type Float%20%28single-precision%29))
  (if (< (Variables|Default|GetCurrentStateTime) 1e+01)
    (bind _output_get (LocalVariables|SetWelcome "Welcome to Snow Day! 
Before you start, you'll need to learn a 
few things."))
    (Rendering|Components|TextRender|SetText (Variables|/Game/VRPlayer/VRBaseBP.VRBaseBP_C|GetHelpText (Variables|Default|GetPlayerPawn_0)) (Utilities|Text|ToText(String) _output_get))
    (else
      (CallFunction|ChangeTutorialState "NewEnumerator2"))))

(fn TeachWaitTrigger
  (params (DeltaTime :type Float%20%28single-precision%29))
  (if (> (Variables|Default|GetTriggerTimesPulled) 5)
    (Default|HighlightTrigger (Variables|/Game/VRPlayer/VRBaseBP.VRBaseBP_C|GetTriggerComponent (Variables|Default|GetPlayerPawn_0)) "Left" false)
    (Default|HighlightTrigger (Variables|/Game/VRPlayer/VRBaseBP.VRBaseBP_C|GetTriggerComponent (Variables|Default|GetPlayerPawn_0)) "Right" false)
    (CallFunction|ChangeTutorialState "NewEnumerator1")))

(fn TeachPickupSnow
  (params (DeltaTime :type Float%20%28single-precision%29))
  (bind _playerpawn_0 (Variables|Default|GetPlayerPawn_0))
  (bind _playerpawn_0_2 (Variables|Default|GetPlayerPawn_0))
  (if (< (Variables|Default|GetCurrentStateTime) 8.0)
    (bind _output_get (LocalVariables|SetPickupSnowText "Good job! In the actual game, you won't 
see a Vive Controller--instead you'll see 
your hands. Go ahead and try pulling the  
trigger to close your hands."))
    (Rendering|Components|TextRender|SetText (Variables|/Game/VRPlayer/VRBaseBP.VRBaseBP_C|GetHelpText (Variables|Default|GetPlayerPawn_0)) (Utilities|Text|ToText(String) _output_get))
    (Rendering|SetVisibility (Variables|/Game/VRPlayer/VRBaseBP.VRBaseBP_C|GetViveControllerRight _playerpawn_0_2) false false)
    (Rendering|Material|SetMaterial (Variables|/Game/VRPlayer/VRBaseBP.VRBaseBP_C|GetLeftHandMesh _playerpawn_0_2) 0 "/Game/Assets/old_mittens/mitten.mitten")
    (elif (< (Variables|Default|GetCurrentStateTime) 11.0)
      (bind _output_get_2 (LocalVariables|SetPickupSnowText "To pick up snow, stick your hand fully into 
a snow-covered object or into the ground. 
Then pull the trigger and hold it. Go ahead 
and give it a try."))
      (Rendering|Components|TextRender|SetText (Variables|/Game/VRPlayer/VRBaseBP.VRBaseBP_C|GetHelpText (Variables|Default|GetPlayerPawn_0)) (Utilities|Text|ToText(String) _output_get_2))
      (Variables|Default|SetAllowPickup true)
      (elif (or (Utilities|IsValid (Variables|/Game/VRPlayer/VRBaseBP.VRBaseBP_C|GetRightGrabbed _playerpawn_0)) (Utilities|IsValid (Variables|/Game/VRPlayer/VRBaseBP.VRBaseBP_C|GetLeftGrabbed _playerpawn_0)))
        (CallFunction|ChangeTutorialState "NewEnumerator3")))))

(fn CheckforGoodThrow
  (params (Condition :type Boolean) (Selection :type EControllerHand%20Enum))
  (bind _playerpawn_0 (Variables|Default|GetPlayerPawn_0))
  (if (not Condition)
    (Variables|Default|SetHasThrown true)
    (switch Utilities|FlowControl|Switch|SwitchonEControllerHand Selection
      (:Left
        (if (> (Math|Vector|VectorLength (Variables|/Script/Snow.VRBase|GetleftHandVelocity _playerpawn_0)) 2e+02)
          (Variables|Default|SetSuccessfulThrow true :!label _label)))
      (:Right
        (if (> (Math|Vector|VectorLength (Variables|/Script/Snow.VRBase|GetrightHandVelocity _playerpawn_0)) 2e+02)
          (goto _label)
          (else
            _)))
      (:Pad
        _)))
  (return))

(fn TeachWaitTeleport
  (params (DeltaTime :type Float%20%28single-precision%29))
  (if (Variables|Default|GetTeleportSuccess)
    (CallFunction|ChangeTutorialState "NewEnumerator9")
    (elif (or (Variables|Default|GetThumbpadRightDown) (Variables|Default|GetThumbpadLeftDown))
      (Rendering|Components|TextRender|SetText (Variables|/Game/VRPlayer/VRBaseBP.VRBaseBP_C|GetHelpText (Variables|Default|GetPlayerPawn_0)) (Utilities|Text|ToText(String) "Notice how a line shoots out of your hand. 
This line indicates where you will teleport. 
If it is red, this indicates that you can't 
teleport to the location you're pointing at. If 
it is green, you can. Point the line around 
until it turns green and release the thumbpad 
button."))
      (else
        (Rendering|Components|TextRender|SetText (Variables|/Game/VRPlayer/VRBaseBP.VRBaseBP_C|GetHelpText (Variables|Default|GetPlayerPawn_0)) (Utilities|Text|ToText(String) "Hold down the thumbpad button. 
"))))))

(fn TutorialPawnSetup
  (params (Controller :type Controller%20Object%20Reference))
  (bind _asvrbase_bp (Utilities|Casting|CastToVRBaseBP (Pawn|GetControlledPawn Controller)))
  (LocalVariables|SettutPawn _asvrbase_bp)
  (Variables|Default|SetPreviousLocation (Transformation|GetWorldLocation (Variables|/Game/VRPlayer/VRBaseBP.VRBaseBP_C|GetHeadCollisionVolume (LocalVariables|GettutPawn))))
  (Default|SetNoobHands (LocalVariables|GettutPawn) true))

(fn HeadHitOverride
  (params (Hit :type Hit%20Result%20Structure) (Snowball :type A%20Snowball%20Replicated%20Object%20Reference) (HitPawn :type VR%20Base%20BP%20Object%20Reference))
  (return true))

(fn MittenHitOverride
  (params (Hit :type Hit%20Result%20Structure) (Snowball :type A%20Snowball%20Replicated%20Object%20Reference) (HitPawn :type VR%20Base%20BP%20Object%20Reference))
  (return false))

(fn TeleportOverride
  (params (TeleportLocation :type Vector :default "0, 0, 0"))
  (return true))

(fn ThumbpadOverride
  (params (ThumbpadComponent :type Thumbpad%20Component%20Object%20Reference) (Pressed :type Boolean) (Hand :type EControllerHand%20Enum :default "Left"))
  (return true))

(fn TriggerOverride
  (params (Pressed :type Boolean) (Hand :type EControllerHand%20Enum :default "Left") (TriggerComponent :type Trigger%20Component%20Object%20Reference))
  (return true))