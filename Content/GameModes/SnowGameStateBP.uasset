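; Game state Blueprint for the snow game mode that clears the scores of inactive players.
; Each tick on the authority, it loops over Players and calls ResetScore on any whose matching PlayersLastActive value exceeds ScoreTimeoutTime.
; The thumbpad and trigger input overrides both return false and perform no actions.
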(event EventBeginPlay)

(event EventTick
  (params (DeltaSeconds :type Float%20%28single-precision%29))
  (Networking|SwitchHasAuthority
    (:Authority
      (for (_array_element _array_index) (Variables|Default|GetPlayers)
        (if (> (Utilities|Array|Get(acopy) (Variables|Default|GetPlayersLastActive) _array_index) (Variables|Default|GetScoreTimeoutTime))
          (Class|SnowGameState|ResetScore _array_element))))))

(fn ConstructionScript)

(fn ThumbpadOverride
  (params (ThumbpadComponent :type Thumbpad%20Component%20Object%20Reference) (Pressed :type Boolean) (Hand :type EControllerHand%20Enum :default "Left"))
  (return false))

(fn TriggerOverride
  (params (Pressed :type Boolean) (Hand :type EControllerHand%20Enum :default "Left") (TriggerComponent :type Trigger%20Component%20Object%20Reference))
  (return false))