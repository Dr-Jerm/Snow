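; Game mode for the Snow Day VR tutorial, teaching walking, teleporting, trigger use, snow pickup and throwing in turn.
; On login, the server spawns and possesses a randomly customized VRBaseBP and registers the player with game state.
; A Tick-driven state machine updates help text, highlights and hand visuals, advancing on time or player actions.
; Trigger, thumbpad and teleport override events gate input by lesson and feed progress back, judging throws by hand speed.
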(event Custom|ChangeTutorialState
  (params (TutState :type TutorialStateEnum%20Enum))
  (Variables|Default|SetPreviousLocation (Transformation|GetWorldLocation (Variables|/Game/VRPlayer/VRBaseBP.VRBaseBP_C|GetHeadCollisionVolume (Variables|Default|GetPlayerPawn))))
  (Variables|Default|SetCurrentStateTime 0.0)
  (Variables|Default|SetTutorialState TutState)
  (Variables|Default|SetTriggerTimesPulled 0))

(event EventTriggerOverride
  (params (Pressed :type Boolean) (Hand :type EControllerHand%20Enum :default "Left") (TriggerComponent :type Trigger%20Component%20Object%20Reference))
  (switch Utilities|FlowControl|Switch|SwitchonTutorialStateEnum (Variables|Default|GetTutorialState)
    (:NewEnumerator8
      (Variables|Default|SetTriggerTimesPulled (+ (Variables|Default|GetTriggerTimesPulled) 1)))
    (:NewEnumerator1
      (if (Variables|Default|GetAllowPickup)
        (Default|TriggerPress TriggerComponent Pressed Hand :!label _label)))
    (:NewEnumerator3
      (CallFunction|CheckforGoodThrow Pressed Hand)
      (goto _label))
    (:NewEnumerator6
      (goto _label))))

(event EventThumbpadOverride
  (params (ThumbpadComponent :type Thumbpad%20Component%20Object%20Reference) (Pressed :type Boolean) (Hand :type EControllerHand%20Enum :default "Left"))
  (switch Utilities|FlowControl|Switch|SwitchonTutorialStateEnum (Variables|Default|GetTutorialState)
    (:NewEnumerator9
      (Default|ThumbPressEvent ThumbpadComponent Pressed Hand :!label _label))
    (:NewEnumerator8
      (goto _label))
    (:NewEnumerator1
      (goto _label))
    (:NewEnumerator3
      (goto _label))
    (:NewEnumerator5
      (Utilities|FlowControl|Sequence
        (:then_0
          (if (and (Variables|Default|GetThumbpadPush) (not (Variables|Default|GetAllowTeleport)))
            (Variables|Default|SetAllowTeleport true)))
        (:then_1
          (if (and (Variables|Default|GetThumbpadPush) (Variables|Default|GetAllowTeleport))
            (goto _label)))))
    (:NewEnumerator10
      (switch Utilities|FlowControl|Switch|SwitchonEControllerHand Hand
        (:Left
          (Variables|Default|SetThumbpadLeftDown Pressed)
          (goto _label))
        (:Right
          (Variables|Default|SetThumbpadRightDown Pressed)
          (goto _label))))
    (:NewEnumerator6
      (goto _label))))

(event EventPostLogin
  (params (NewPlayer :type Player%20Controller%20Object%20Reference))
  (Networking|SwitchHasAuthority
    (:Authority
      (bind _asbase_player_controller_bp (Utilities|Casting|CastToBasePlayerControllerBP NewPlayer))
      (bind _outactors (Actor|GetAllActorsOfClass "/Script/Engine.PlayerStart"))
      (bind _returnvalue (Game|SpawnActorfromClass "/Game/VRPlayer/VRBaseBP.VRBaseBP_C" (Math|Conversions|ToTransform(Vector) (Transformation|GetActorLocation (Utilities|Array|Get(acopy) _outactors (Math|Integer|%(Integer) (Variables|Default|GetSpawnOrder) (Utilities|Array|Length _outactors))))) "AlwaysSpawn" 0 0))
      (Pawn|Possess _asbase_player_controller_bp _returnvalue)
      (Default|ClientPostLogin _asbase_player_controller_bp)
      (Variables|/Script/Snow.VRBase|SetCustomization _returnvalue (Utilities|Array|MakeArray (Math|Integer|%(Integer) (Math|Random|RandomInteger 10) 2) (Math|Integer|%(Integer) (Math|Random|RandomInteger 10) 2) (Math|Integer|%(Integer) (Math|Random|RandomInteger 10) 2) (Math|Integer|%(Integer) (Math|Random|RandomInteger 10) 2) (Math|Integer|%(Integer) (Math|Random|RandomInteger 10) 2)))
      (Default|VisualChange _returnvalue)
      (bind _assnow_game_state_bp (Utilities|Casting|CastToSnowGameStateBP (Game|GetGameState)))
      (bind _assnow_player_state_bp (Utilities|Casting|CastToSnowPlayerStateBP (Variables|/Script/Engine.Controller|GetPlayerState _asbase_player_controller_bp)))
      (bind _playerscoreindex (Class|SnowGameState|PlayerJoin _assnow_game_state_bp (Variables|/Script/Engine.PlayerState|GetPlayerId _assnow_player_state_bp)))
      (Variables|/Script/Snow.SnowPlayerState|SetScoreIndex _assnow_player_state_bp _playerscoreindex)
      (Variables|Default|SetSpawnOrder (+ (Variables|Default|GetSpawnOrder) 1))
      (Variables|/Game/VRPlayer/SnowPlayerStateBP.SnowPlayerStateBP_C|SetpawnReference _assnow_player_state_bp _returnvalue))))

(event EventTeleportOverride
  (params (TeleportLocation :type Vector))
  (Variables|Default|SetTeleportSuccess true)
  (Default|RoomScaleTeleport (Variables|Default|GetPlayerPawn) TeleportLocation))

(event EventTick
  (params (DeltaSeconds :type Float%20%28single-precision%29))
  (Variables|Default|SetDeltaTime DeltaSeconds)
  (Variables|Default|SetCurrentStateTime (+ (Variables|Default|GetDeltaTime) (Variables|Default|GetCurrentStateTime)))
  (Variables|Default|SetThumbpadPush false)
  (switch Utilities|FlowControl|Switch|SwitchonTutorialStateEnum (Variables|Default|GetTutorialState)
    (:NewEnumerator7
      (CallFunction|TeachWelcome (Variables|Default|GetDeltaTime)))
    (:NewEnumerator2
      (CallFunction|TeachWalkAround (Variables|Default|GetDeltaTime)))
    (:NewEnumerator9
      (CallFunction|TeachPullTrigger (Variables|Default|GetDeltaTime)))
    (:NewEnumerator8
      (CallFunction|TeachWaitTrigger (Variables|Default|GetDeltaTime)))
    (:NewEnumerator1
      (CallFunction|TeachPickupSnow (Variables|Default|GetDeltaTime)))
    (:NewEnumerator3
      (CallFunction|TeachThrowSnow (Variables|Default|GetDeltaTime)))
    (:NewEnumerator5
      (CallFunction|TeachTeleport (Variables|Default|GetDeltaTime)))
    (:NewEnumerator10
      (CallFunction|TeachWaitTeleport (Variables|Default|GetDeltaTime)))
    (:NewEnumerator6
      (CallFunction|TeachDone (Variables|Default|GetDeltaTime)))))

(event EventBeginPlay
  (bind _asvrbase_bp (Utilities|Casting|CastToVRBaseBP (Game|Player|GetPlayerPawn 0)))
  (Variables|Default|SetPlayerPawn _asvrbase_bp)
  (Rendering|SetVisibility (Variables|/Game/VRPlayer/VRBaseBP.VRBaseBP_C|GetViveControllerRight (Variables|Default|GetPlayerPawn)) true false)
  (Variables|Default|SetPreviousLocation (Transformation|GetWorldLocation (Variables|/Game/VRPlayer/VRBaseBP.VRBaseBP_C|GetHeadCollisionVolume (Variables|Default|GetPlayerPawn))))
  (Rendering|Material|SetMaterial (Variables|/Game/VRPlayer/VRBaseBP.VRBaseBP_C|GetRightHandMesh (Variables|Default|GetPlayerPawn)) 0 "/Game/Assets/new_mittens/WireframeMitten.WireframeMitten")
  (Rendering|Material|SetMaterial (Variables|/Game/VRPlayer/VRBaseBP.VRBaseBP_C|GetLeftHandMesh (Variables|Default|GetPlayerPawn)) 0 "/Game/Assets/new_mittens/WireframeMitten.WireframeMitten"))

(fn ConstructionScript)

(fn TeachWalkAround
  (params (DeltaTime :type Float%20%28single-precision%29))
  (bind _playerpawn (Variables|Default|GetPlayerPawn))
  (bind _headcollisionvolume (Variables|/Game/VRPlayer/VRBaseBP.VRBaseBP_C|GetHeadCollisionVolume _playerpawn))
  (bind _returnvalue (Transformation|GetWorldLocation _headcollisionvolume))
  (Utilities|FlowControl|Sequence
    (:then_0
      (if (> (Math|Vector|VectorLength (- (Variables|Default|GetPreviousLocation) _returnvalue)) 0.1)
        (Variables|Default|SetTotalDistanceTraveled (+ (Math|Vector|VectorLength (- (Variables|Default|GetPreviousLocation) _returnvalue)) (Variables|Default|GetTotalDistanceTraveled)))
        (Variables|Default|SetPreviousLocation _returnvalue)))
    (:then_1
      (if (< (Variables|Default|GetTotalDistanceTraveled) 2.5e+02)
        (bind _output_get (LocalVariables|SetPlayerText "To walk around, simply walk around 
as you would in real life. If you see a 
grid appear, you've gone too far! Go 
ahead and try walking within the grid."))
        (Rendering|Components|TextRender|SetText (Variables|/Game/VRPlayer/VRBaseBP.VRBaseBP_C|GetHelpText (Variables|Default|GetPlayerPawn)) (Utilities|Text|ToText(String) _output_get))
        (elif (< (Variables|Default|GetTotalDistanceTraveled) 5e+02)
          (bind _output_get_2 (LocalVariables|SetPlayerText "Keep going! You're almost there! 
Remember you can also turn your 
body to look around."))
          (Rendering|Components|TextRender|SetText (Variables|/Game/VRPlayer/VRBaseBP.VRBaseBP_C|GetHelpText (Variables|Default|GetPlayerPawn)) (Utilities|Text|ToText(String) _output_get_2))
          (else
            (CallFunction|ChangeTutorialState "NewEnumerator5")))))))

(fn TeachPullTrigger
  (params (DeltaTime :type Float%20%28single-precision%29))
  (bind _playerpawn (Variables|Default|GetPlayerPawn))
  (bind _triggercomponent (Variables|/Game/VRPlayer/VRBaseBP.VRBaseBP_C|GetTriggerComponent _playerpawn))
  (if (< (Variables|Default|GetCurrentStateTime) 1e+01)
    (bind _output_get (LocalVariables|SetPlayerText "Next, you're going to learn to pick 
up snow. Look at your controllers. 
You'll see two highlighted buttons on 
the bottom. (You might need to rotate 
your controllers a bit.)"))
    (Rendering|Components|TextRender|SetText (Variables|/Game/VRPlayer/VRBaseBP.VRBaseBP_C|GetHelpText (Variables|Default|GetPlayerPawn)) (Utilities|Text|ToText(String) _output_get))
    (Default|HighlightTrigger _triggercomponent "Left" true)
    (Default|HighlightTrigger _triggercomponent "Right" true)
    (else
      (bind _output_get_2 (LocalVariables|SetPlayerText "These buttons are called triggers. 
Use your forefinger to give each 
of them a few squeezes."))
      (Rendering|Components|TextRender|SetText (Variables|/Game/VRPlayer/VRBaseBP.VRBaseBP_C|GetHelpText (Variables|Default|GetPlayerPawn)) (Utilities|Text|ToText(String) _output_get_2))
      (CallFunction|ChangeTutorialState "NewEnumerator8"))))

(fn TeachThrowSnow
  (params (DeltaTime :type Float%20%28single-precision%29))
  (if (Variables|Default|GetHasThrown)
    (if (Variables|Default|GetSuccessfulThrow)
      (CallFunction|ChangeTutorialState "NewEnumerator6")
      (else
        (bind _output_get (LocalVariables|SetHelpText "Nice try, but you'll need to try throwing 
harder than that if you expect to hit 
anybody. Pick up another snowball 
and try again."))
        (Rendering|Components|TextRender|SetText (Variables|/Game/VRPlayer/VRBaseBP.VRBaseBP_C|GetHelpText (Variables|Default|GetPlayerPawn)) (Utilities|Text|ToText(String) _output_get))))
    (else
      (bind _output_get_2 (LocalVariables|SetHelpText "Radical! Now, make a throwing motion and 
let go of the snowball. "))
      (Rendering|Components|TextRender|SetText (Variables|/Game/VRPlayer/VRBaseBP.VRBaseBP_C|GetHelpText (Variables|Default|GetPlayerPawn)) (Utilities|Text|ToText(String) _output_get_2)))))

(fn TeachTeleport
  (params (DeltaTime :type Float%20%28single-precision%29))
  (bind _playerpawn (Variables|Default|GetPlayerPawn))
  (bind _thumbpadcomponent (Variables|/Game/VRPlayer/VRBaseBP.VRBaseBP_C|GetThumbpadComponent _playerpawn))
  (if (< (Variables|Default|GetCurrentStateTime) 1e+01)
    (bind _output_get (LocalVariables|SetTeleportString "Nice walking! Walking and turning around is 
great, but sometimes you'll need to cover 
more distance. That's where teleporting  
comes in."))
    (Rendering|Components|TextRender|SetText (Variables|/Game/VRPlayer/VRBaseBP.VRBaseBP_C|GetHelpText (Variables|Default|GetPlayerPawn)) (Utilities|Text|ToText(String) _output_get))
    (elif (< (Variables|Default|GetCurrentStateTime) 11.0)
      (bind _output_get_2 (LocalVariables|SetTeleportString "Take a look at your controller.  
You'll see a big round button  
that's highlighted in yellow. Go 
ahead and press it."))
      (Rendering|Components|TextRender|SetText (Variables|/Game/VRPlayer/VRBaseBP.VRBaseBP_C|GetHelpText _playerpawn) (Utilities|Text|ToText(String) _output_get_2))
      (Default|HighlightThumbpad _thumbpadcomponent "Left" true)
      (Default|HighlightThumbpad _thumbpadcomponent "Right" true)
      (else
        (Variables|Default|SetThumbpadPush true)
        (if (Variables|Default|GetAllowTeleport)
          (Default|HighlightThumbpad _thumbpadcomponent "Left" false)
          (Default|HighlightThumbpad _thumbpadcomponent "Right" false)
          (CallFunction|ChangeTutorialState "NewEnumerator10"))))))

(fn TeachDone
  (params (DeltaTime :type Float%20%28single-precision%29))
  (Rendering|Components|TextRender|SetText (Variables|/Game/VRPlayer/VRBaseBP.VRBaseBP_C|GetHelpText (Variables|Default|GetPlayerPawn)) (Utilities|Text|ToText(String) "Great job! You're ready for a real snow 
brawl. Go get 'em!")))

(fn TeachWelcome
  (params (DeltaTime :type Float%20%28single-precision%29))
  (if (< (Variables|Default|GetCurrentStateTime) 1e+01)
    (bind _output_get (LocalVariables|SetWelcome "Welcome to Snow Day! 
Before you start, you'll need to learn a 
few things."))
    (Rendering|Components|TextRender|SetText (Variables|/Game/VRPlayer/VRBaseBP.VRBaseBP_C|GetHelpText (Variables|Default|GetPlayerPawn)) (Utilities|Text|ToText(String) _output_get))
    (else
      (CallFunction|ChangeTutorialState "NewEnumerator2"))))

(fn TeachWaitTrigger
  (params (DeltaTime :type Float%20%28single-precision%29))
  (if (> (Variables|Default|GetTriggerTimesPulled) 5)
    (Default|HighlightTrigger (Variables|/Game/VRPlayer/VRBaseBP.VRBaseBP_C|GetTriggerComponent (Variables|Default|GetPlayerPawn)) "Left" false)
    (Default|HighlightTrigger (Variables|/Game/VRPlayer/VRBaseBP.VRBaseBP_C|GetTriggerComponent (Variables|Default|GetPlayerPawn)) "Right" false)
    (CallFunction|ChangeTutorialState "NewEnumerator1")))

(fn TeachPickupSnow
  (params (DeltaTime :type Float%20%28single-precision%29))
  (bind _playerpawn (Variables|Default|GetPlayerPawn))
  (bind _playerpawn_2 (Variables|Default|GetPlayerPawn))
  (if (< (Variables|Default|GetCurrentStateTime) 1e+01)
    (bind _output_get (LocalVariables|SetPickupSnowText "Good job! You might have noticed that 
the gloves closed when you pulled the 
trigger. "))
    (Rendering|Components|TextRender|SetText (Variables|/Game/VRPlayer/VRBaseBP.VRBaseBP_C|GetHelpText (Variables|Default|GetPlayerPawn)) (Utilities|Text|ToText(String) _output_get))
    (elif (< (Variables|Default|GetCurrentStateTime) 2e+01)
      (bind _output_get_2 (LocalVariables|SetPickupSnowText "In the actual game, you won't see 
a Vive Controller--instead you'll see your 
hands. Go ahead and try pulling the  
trigger to close your hands."))
      (Rendering|Components|TextRender|SetText (Variables|/Game/VRPlayer/VRBaseBP.VRBaseBP_C|GetHelpText (Variables|Default|GetPlayerPawn)) (Utilities|Text|ToText(String) _output_get_2))
      (Rendering|SetVisibility (Variables|/Game/VRPlayer/VRBaseBP.VRBaseBP_C|GetViveControllerRight _playerpawn_2) false false)
      (Rendering|Material|SetMaterial (Variables|/Game/VRPlayer/VRBaseBP.VRBaseBP_C|GetLeftHandMesh _playerpawn_2) 0 "/Game/Assets/mittens/mitten.mitten")
      (elif (< (Variables|Default|GetCurrentStateTime) 21.0)
        (bind _output_get_3 (LocalVariables|SetPickupSnowText "To pick up snow, stick your hand fully into 
a snow-covered object or into the ground. 
Then pull the trigger and hold it. Go ahead 
and give it a try."))
        (Rendering|Components|TextRender|SetText (Variables|/Game/VRPlayer/VRBaseBP.VRBaseBP_C|GetHelpText (Variables|Default|GetPlayerPawn)) (Utilities|Text|ToText(String) _output_get_3))
        (Variables|Default|SetAllowPickup true)
        (elif (or (Utilities|IsValid (Variables|/Game/VRPlayer/VRBaseBP.VRBaseBP_C|GetRightGrabbed _playerpawn)) (Utilities|IsValid (Variables|/Game/VRPlayer/VRBaseBP.VRBaseBP_C|GetLeftGrabbed _playerpawn)))
          (CallFunction|ChangeTutorialState "NewEnumerator3"))))))

(fn CheckforGoodThrow
  (params (Condition :type Boolean) (Selection :type EControllerHand%20Enum))
  (bind _playerpawn (Variables|Default|GetPlayerPawn))
  (if (not Condition)
    (Variables|Default|SetHasThrown true)
    (switch Utilities|FlowControl|Switch|SwitchonEControllerHand Selection
      (:Left
        (if (> (Math|Vector|VectorLength (Variables|/Script/Snow.VRBase|GetleftHandVelocity _playerpawn)) 2e+02)
          (Variables|Default|SetSuccessfulThrow true :!label _label)))
      (:Right
        (if (> (Math|Vector|VectorLength (Variables|/Script/Snow.VRBase|GetrightHandVelocity _playerpawn)) 2e+02)
          (goto _label)
          (else
            _)))
      (:Pad
        _)))
  (return))

(fn TeachWaitTeleport
  (params (DeltaTime :type Float%20%28single-precision%29))
  (if (Variables|Default|GetTeleportSuccess)
    (CallFunction|ChangeTutorialState "NewEnumerator9")
    (elif (or (Variables|Default|GetThumbpadRightDown) (Variables|Default|GetThumbpadLeftDown))
      (Rendering|Components|TextRender|SetText (Variables|/Game/VRPlayer/VRBaseBP.VRBaseBP_C|GetHelpText (Variables|Default|GetPlayerPawn)) (Utilities|Text|ToText(String) "Notice how a line shoots out of your hand. 
This line indicates where you will teleport. 
If it is red, this indicates that you can't 
teleport to the location you're pointing at. If 
it is green, you can. Point the line around 
until it turns green and release the thumbpad 
button."))
      (else
        (Rendering|Components|TextRender|SetText (Variables|/Game/VRPlayer/VRBaseBP.VRBaseBP_C|GetHelpText (Variables|Default|GetPlayerPawn)) (Utilities|Text|ToText(String) "Hold down the thumbpad button. 
"))))))