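; Base grabbable hat Blueprint that lets a character change the hat they wear by releasing one at their head.
; On release, it searches its Sphere's overlapping components for the releaser's head collision volume.
; A match copies the grabbable's static mesh onto the releaser's Hat component.
; The actor destroys itself after every release, whether or not the hat was applied.
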(event EventBeginPlay)

(event EventTick
  (params (DeltaSeconds :type Float%20%28single-precision%29))
  (|CallParentFunction DeltaSeconds))

(event EventBeReleased
  (params (Releaser :type VR%20Base%20BP%20Object%20Reference) (Hand :type EControllerHand%20Enum :default "Left") (Velocity :type Vector) (Location :type Vector))
  (|CallParentFunction Releaser Hand Velocity Location)
  (bind _array_element (Utilities|Array|ForEachLoopwithBreak (Class|PrimitiveComponent|GetOverlappingComponents (Variables|Default|GetSphere)) :!label _label)
    (:LoopBody
      (if (== _array_element (Variables|/Game/VRBaseBP.VRBaseBP_C|GetHeadCollisionVolume Releaser))
        (Components|StaticMesh|SetStaticMesh (Variables|/Game/VRBaseBP.VRBaseBP_C|GetHat Releaser) (Variables|/Script/Engine.StaticMeshComponent|GetStaticMesh (Variables|Default|GetStaticMesh)))
        (goto _label Break)))
    (:Completed
      (Actor|DestroyActor))))

(event Collision|EventActorEndOverlap
  (params (OtherActor :type Actor%20Object%20Reference)))

(fn ConstructionScript
  (|CallParentFunction))