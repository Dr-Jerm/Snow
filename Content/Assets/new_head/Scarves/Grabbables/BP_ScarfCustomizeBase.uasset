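; BP_ScarfCustomizeBase is a grabbable scarf that customizes a character when released on the head.
; On release, overlap between its Sphere and the releaser's HeadCollisionVolume copies the scarf mesh onto the Chin component.
; It then respawns by spawning a base-class copy with the same mesh at its BeginPlay location and destroying itself.
; A missed drop does the same after a delay if IsDropped is still set.
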(event EventBeginPlay
  (Variables|Default|SetStartLocation (Transformation|GetActorLocation)))

(event EventTick
  (params (DeltaSeconds :type Float%20%28single-precision%29))
  (|CallParentFunction DeltaSeconds))

(event EventBeReleased
  (params (Releaser :type VR%20Base%20BP%20Object%20Reference) (Hand :type EControllerHand%20Enum :default "Left") (Velocity :type Vector) (Location :type Vector))
  (|CallParentFunction Releaser Hand Velocity Location)
  (bind _array_element (Utilities|Array|ForEachLoopwithBreak (Class|PrimitiveComponent|GetOverlappingComponents (Variables|Default|GetSphere)) :!label _label)
    (:LoopBody
      (if (== _array_element (Variables|/Game/VRBaseBP.VRBaseBP_C|GetHeadCollisionVolume Releaser))
        (Components|StaticMesh|SetStaticMesh (Variables|/Game/VRBaseBP.VRBaseBP_C|GetChin Releaser) (Variables|/Script/Engine.StaticMeshComponent|GetStaticMesh (Variables|Default|GetStaticMesh)))
        (Variables|Default|SetisPlaced true)
        (goto _label Break)))
    (:Completed
      (if (Variables|Default|GetisPlaced)
        (bind _returnvalue (Game|SpawnActorfromClass "BP_ScarfCustomizeBase_C" (Math|Transform|MakeTransform (Variables|Default|GetStartLocation)) "Undefined" 0 0 :!label _label_2))
        (Components|StaticMesh|SetStaticMesh (Variables|/Game/TestThrowable.TestThrowable_C|GetStaticMesh _returnvalue) (Variables|/Script/Engine.StaticMeshComponent|GetStaticMesh (Variables|Default|GetStaticMesh)))
        (Actor|DestroyActor)
        (else
          (Variables|Default|SetisDropped true)
          (Utilities|FlowControl|Delay 5.0)
          (if (Variables|Default|GetisDropped)
            (goto _label_2)))))))

(event Collision|EventActorEndOverlap
  (params (OtherActor :type Actor%20Object%20Reference)))

(fn ConstructionScript
  (|CallParentFunction))