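; Grabbable VR hat that the player wears by releasing it over their head.
; On release, a sphere overlap with the player's head collision volume copies the hat's mesh onto the player's hat component.
; A placed hat, or one left dropped after a short delay, respawns by spawning a base-class copy with the same mesh at its start location and destroying itself.
; Grabbing it again clears the dropped flag.
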(event EventBeginPlay
  (Variables|Default|SetStartLocation (Transformation|GetActorLocation)))

(event EventBeGrabbed
  (params (Grabber :type Pawn%20Object%20Reference) (Hand :type EControllerHand%20Enum :default "Left") (GrabLocation :type Vector))
  (|CallParentFunction Grabber Hand GrabLocation)
  (Variables|Default|SetisDropped false))

(event EventTick
  (params (DeltaSeconds :type Float%20%28single-precision%29))
  (|CallParentFunction DeltaSeconds))

(event EventBeReleased
  (params (Releaser :type Pawn%20Object%20Reference) (Hand :type EControllerHand%20Enum :default "Left") (Velocity :type Vector) (Location :type Vector) (RelaseTime :type Float%20%28single-precision%29))
  (|CallParentFunction Releaser Hand Velocity Location 0.0)
  (bind _asvrbase_bp (Utilities|Casting|CastToVRBaseBP Releaser))
  (bind _array_element (Utilities|Array|ForEachLoopwithBreak (Class|PrimitiveComponent|GetOverlappingComponents (Variables|Default|GetSphere)) :!label _label)
    (:LoopBody
      (if (== _array_element (Variables|/Game/VRPlayer/VRBaseBP.VRBaseBP_C|GetHeadCollisionVolume _asvrbase_bp))
        (Components|StaticMesh|SetStaticMesh (Variables|/Game/VRPlayer/VRBaseBP.VRBaseBP_C|GetHat_static _asvrbase_bp) (Variables|/Script/Engine.StaticMeshComponent|GetStaticMesh (Variables|Default|GetStaticMesh)))
        (Variables|Default|SetisPlaced true)
        (goto _label Break)))
    (:Completed
      (if (Variables|Default|GetisPlaced)
        (bind _returnvalue (Game|SpawnActorfromClass "BP_HatCustomizeBase_C" (Math|Transform|MakeTransform (Variables|Default|GetStartLocation)) "Undefined" 0 0 :!label _label_2))
        (Components|StaticMesh|SetStaticMesh (Variables|/Game/TestThrowable.TestThrowable_C|GetStaticMesh _returnvalue) (Variables|/Script/Engine.StaticMeshComponent|GetStaticMesh (Variables|Default|GetStaticMesh)))
        (Actor|DestroyActor)
        (else
          (Variables|Default|SetisDropped true)
          (Utilities|FlowControl|Delay 5.0)
          (if (Variables|Default|GetisDropped)
            (goto _label_2)))))))

(event Collision|EventActorEndOverlap
  (params (OtherActor :type Actor%20Object%20Reference)))

(fn ConstructionScript
  (|CallParentFunction))