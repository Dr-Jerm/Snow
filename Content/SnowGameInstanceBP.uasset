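; SnowGameInstanceBP is a game instance Blueprint that handles online session invites and connection error reporting.
; Both receiving and accepting an invite immediately call JoinSession for the local player's controller, then print the inviter's net ID on success.
; Network and travel error events only print the failure type, plus the server flag for network errors, and Init prints a startup message.
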(event EventInit
  (Development|PrintText "SnowGameInstance initialized!"))

(event EventOnSessionInviteReceived
  (params (LocalPlayerNum :type Integer) (PersonInviting :type BP%20Unique%20Net%20Id%20Structure) (AppId :type String) (SessionToJoin :type Blueprint%20Session%20Result%20Structure%20%28by%20ref%29))
  (|JoinSession (Game|GetPlayerController LocalPlayerNum) SessionToJoin
    (:OnSuccess
      (Development|PrintText (Utilities|Text|ToText(String) (Utilities|String|Append "Recieved invite from: " (Class|AdvancedSessionsLibrary|UniqueNetIdtoString PersonInviting)))))))

(event EventOnSessionInviteAccepted
  (params (LocalPlayerNum :type Integer) (PersonInviting :type BP%20Unique%20Net%20Id%20Structure) (SessionToJoin :type Blueprint%20Session%20Result%20Structure%20%28by%20ref%29))
  (|JoinSession (Game|GetPlayerController LocalPlayerNum) SessionToJoin
    (:OnSuccess
      (Development|PrintText (Utilities|Text|ToText(String) (Utilities|String|Append "Accepting invite from: " (Class|AdvancedSessionsLibrary|UniqueNetIdtoString PersonInviting)))))))

(event EventHandleNetworkError
  (params (FailureType :type ENetworkFailure%20Enum) (bIsServer :type Boolean))
  (Development|PrintText (Utilities|Text|ToText(String) (Utilities|String|Append "Network failure type: " (Utilities|String|EnumtoString FailureType) " Is server: " (Utilities|String|ToString(Boolean) bIsServer))) false true "(R=1.000000,G=0.007345,B=0.000000,A=1.000000)"))

(event EventHandleTravelError
  (params (FailureType :type ETravelFailure%20Enum))
  (Development|PrintText (Utilities|Text|ToText(String) (Utilities|String|Append "Travel failure type: " (Utilities|String|EnumtoString FailureType))) false true "(R=1.000000,G=0.007345,B=0.000000,A=1.000000)"))