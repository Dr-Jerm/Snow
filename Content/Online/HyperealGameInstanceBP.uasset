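; Game instance that authorizes the Hypereal user at startup, quitting on failure, and manages online multiplayer sessions.
; Search, join, host and leave events run through a SetState guard on OnlineState that rejects re-entering the current state.
; Search can auto-join the best result; join and leave destroy any existing session first, continuing even on failure.
; Level changes use seamless ServerTravel when player controllers exist, otherwise open a listen-server level.
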(event EventSessionServerTravel
  (params (level :type Name))
  (bind _returnvalue (Utilities|Text|ToText(Name) level))
  (bind _result (Utilities|Text|FormatText "ServerTravel {level}?listen" _returnvalue))
  (bind _returnvalue_2 (Utilities|String|ToString(Text) _result))
  (Development|PrintText "SERVER TRAVEL")
  (bind _assnow_game_mode_bp (Utilities|Casting|CastToSnowGameModeBP (Game|GetGameMode))
    (:then
      (Variables|/Game/GameModes/SnowGameModeBP.SnowGameModeBP_C|SetServerTravelling _assnow_game_mode_bp true))
    (:CastFailed
      _))
  (bind _outactors (Actor|GetAllActorsOfClass "/Game/VRPlayer/BasePlayerControllerBP.BasePlayerControllerBP_C"))
  (if (> (Utilities|Array|Length _outactors) 0)
    (Variables|/Script/Engine.GameMode|SetbUseSeamlessTravel _assnow_game_mode_bp true)
    (Development|PrintString _returnvalue_2)
    (Development|ExecuteConsoleCommand _returnvalue_2)
    (else
      (Game|OpenLevel(byName) level true "listen"))))

(event EventSearchSessions
  (params (autoJoin :type Boolean))
  (Utilities|SetState "OS_Searching"
    (:NewState
      (bind _results (|FindSessions (Game|GetPlayerController 0) 15 false)
        (:OnSuccess
          (Utilities|SetState "OS_Results"
            (:NewState
              (bind _output_get (Variables|Default|SetCachedSessions _results))
              (if (> (Utilities|Array|Length _output_get) 0)
                (if autoJoin
                  (bind _session (Class|SnowGameInstance|SelectBestSession))
                  (Class|SnowGameInstance|JoinSession _session))
                (else
                  (Utilities|SetState "OS_None_Found"))))))
        (:OnFailure
          (Variables|Default|SetErrorMessage "Failed to Find Hypereal Sessions")
          (Utilities|SetState "OS_Error"))))))

(event EventJoinSession
  (params (session :type Blueprint%20Session%20Result%20Structure))
  (|DestroySession (Game|GetPlayerController 0)
    (:OnSuccess
      _)
    (:OnFailure
      _))
  (if (Class|AdvancedSessionsLibrary|IsValidSession session)
    (Utilities|SetState "OS_Joining"
      (:NewState
        (Development|PrintText (Utilities|Text|ToText(String) (Utilities|String|Append "Attempting to join: " "Hypereal Session")))
        (|JoinSession (Game|GetPlayerController 0) session
          (:OnSuccess
            (Development|PrintText (Utilities|Text|ToText(String) (Utilities|String|Append "Joining session on server: " (Class|FindSessionsCallbackProxy|GetServerName session))))
            (Utilities|SetState "OS_Joining"))
          (:OnFailure
            (Development|PrintString "Failed to Join Hypereal Session")))))
    (else
      (Variables|Default|SetErrorMessage "Session not valid!")
      (Utilities|SetState "OS_Error"))))

(event EventInit
  (|VerifyUserAuthorization
    (:then
      (|CallParentFunction))
    (:OnSuccess
      (Development|PrintString "Hypereal User Authorized")
      (bind (_hyperealuserid _hyperealusername) (|GetHyperealIdentity)
        (:OnSuccess
          (Development|PrintText (Utilities|Text|FormatText "Hypereal User {name} with ID: {id} correctly identified" (Utilities|Text|ToText(String) _hyperealusername) (Utilities|Text|ToText(String) _hyperealuserid)))
          (Class|HyperealPlatformUtilsLibrary|SetPlayerUniqueId (Game|GetPlayerController 0)))
        (:OnFailure
          (Development|PrintString "ERROR: Hypereal User Failed Identity GET"))))
    (:OnFailure
      (Development|PrintString "ERROR: Hypereal User Failed Authorization")
      (Utilities|FlowControl|Delay 1e+01)
      (Game|QuitGame 0 "Quit"))))

(event EventLeaveSession
  (params (level :type Name))
  (|DestroySession (Game|GetPlayerController 0)
    (:OnSuccess
      _)
    (:OnFailure
      _))
  (Utilities|SetState "OS_Offline"
    (:NewState
      _)
    (:SameState
      _))
  (if (or (== (Utilities|String|Len (Utilities|String|ToString(Name) level)) 0) (Utilities|Enum|Equal(Enum) (Utilities|String|ToString(Name) level) "None"))
    (Game|OpenLevel(byName) "SNW_entry")
    (else
      (Game|OpenLevel(byName) level))))

(event EventHostSession
  (params (level :type Name))
  (|Session (Game|GetPlayerController 0) 6 false
    (:OnSuccess
      (Utilities|SetState "OS_Hosting"
        (:NewState
          (Game|OpenLevel(byName) level true "listen")
          (Development|PrintText "Session Started" false))))
    (:OnFailure
      (Variables|Default|SetErrorMessage "Failed to Host Hypereal Session")
      (Utilities|SetState "OS_Error"))))