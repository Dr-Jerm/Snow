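; Game instance that manages online multiplayer sessions through Advanced Sessions: hosting listen servers, searching, joining, invites and leaving.
; A SetState macro tracks the online state and flags re-entry, gating search and join.
; Search can auto-join the first valid result; its hosting fallback sits only on the empty-result Same State branch.
; Network errors, travel errors and shutdown destroy the session, then open the entry level, even if destruction fails.
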(event EventShutdown
  (CallFunction|LeaveSession "None"))

(event EventInit
  (Development|PrintText "SnowGameInstance initialized!" false))

(event EventOnSessionInviteReceived
  (params (LocalPlayerNum :type Integer) (PersonInviting :type BP%20Unique%20Net%20Id%20Structure) (AppId :type String) (SessionToJoin :type Blueprint%20Session%20Result%20Structure%20%28by%20ref%29))
  (|JoinSession (Game|GetPlayerController LocalPlayerNum) SessionToJoin
    (:OnSuccess
      (Development|PrintText (Utilities|Text|ToText(String) (Utilities|String|Append "Recieved invite from: " (Class|AdvancedSessionsLibrary|UniqueNetIdtoString PersonInviting)))))))

(event EventOnSessionInviteAccepted
  (params (LocalPlayerNum :type Integer) (PersonInviting :type BP%20Unique%20Net%20Id%20Structure) (SessionToJoin :type Blueprint%20Session%20Result%20Structure%20%28by%20ref%29))
  (|JoinSession (Game|GetPlayerController LocalPlayerNum) SessionToJoin
    (:OnSuccess
      (Development|PrintText (Utilities|Text|ToText(String) (Utilities|String|Append "Accepting invite from: " (Class|AdvancedSessionsLibrary|UniqueNetIdtoString PersonInviting)))))))

(event EventHandleNetworkError
  (params (FailureType :type ENetworkFailure%20Enum :default "NetDriverAlreadyExists") (bIsServer :type Boolean))
  (Development|PrintText (Utilities|Text|ToText(String) (Utilities|String|Append "Network failure type: " (Utilities|String|EnumtoString FailureType) " Is server: " (Utilities|String|ToString(Boolean) bIsServer) " Leaving session.")) false true "(R=1.000000,G=0.007345,B=0.000000,A=1.000000)")
  (CallFunction|LeaveSession "None"))

(event EventHandleTravelError
  (params (FailureType :type ETravelFailure%20Enum :default "NoLevel"))
  (Development|PrintText (Utilities|Text|ToText(String) (Utilities|String|Append "Travel failure type: " (Utilities|String|EnumtoString FailureType) " Leaving Session.")) false true "(R=1.000000,G=0.007345,B=0.000000,A=1.000000)")
  (CallFunction|LeaveSession "None"))

(event Custom|HostGame
  (params (level :type Name))
  (if (Ability|HasAuthority (Game|GetPlayerController 0))
    (|AdvancedSession 0 (Game|GetPlayerController 0) 12 0 (Variables|Default|GetLAN) true false true true false false false true
      (:OnSuccess
        (Game|OpenLevel(byName) level true "listen")
        (Utilities|SetState "NewEnumerator4"
          (:NewState
            (Development|PrintText "Session Started" false))))
      (:OnFailure
        (Variables|Default|SetErrorMessage "Error Hosting Game!")
        (Utilities|SetState "NewEnumerator5")))
    (else
      (Variables|Default|SetErrorMessage "Not Authorized to host")
      (Utilities|SetState "NewEnumerator5"))))

(event Custom|FindSessions
  (params (shouldAutoJoin :type Boolean))
  (Utilities|SetState "NewEnumerator1"
    (:NewState
      (bind _results (|FindSessionsAdvanced (Game|GetPlayerController 0) 4 (Variables|Default|GetLAN) "ClientServersOnly")
        (:OnSuccess
          (bind _output_get (Variables|Default|SetLastSessionSearchResults _results))
          (if (!= (Utilities|Array|Length _output_get) 0)
            (Utilities|SetState "NewEnumerator2"
              (:SameState
                _)
              (:NewState
                _))
            (if shouldAutoJoin
              (bind _foundsession (CallFunction|SelectBestSession))
              (CallFunction|JoinSession _foundsession))
            (else
              (Utilities|SetState "NewEnumerator7"
                (:SameState
                  (if shouldAutoJoin
                    (CallFunction|HostGame "BRL_rag")))))))
        (:OnFailure
          (Variables|Default|SetErrorMessage "Failed to find sessions")
          (Utilities|SetState "NewEnumerator5"))))))

(event Custom|JoinSession
  (params (sessionRef :type Blueprint%20Session%20Result%20Structure))
  (Utilities|SetState "NewEnumerator8"
    (:NewState
      (if (Class|AdvancedSessionsLibrary|IsValidSession sessionRef)
        (Development|PrintText (Utilities|Text|ToText(String) (Utilities|String|Append "Attempting to join: " (Utilities|SessiontoString sessionRef))))
        (|JoinSession (Game|GetPlayerController 0) sessionRef
          (:OnSuccess
            (Utilities|SetState "NewEnumerator3"
              (:NewState
                (Development|PrintText (Utilities|Text|ToText(String) (Utilities|String|Append "Joining session on server: " (Class|FindSessionsCallbackProxy|GetServerName sessionRef)))))))
          (:OnFailure
            (Variables|Default|SetErrorMessage "Error Hosting Game!")
            (Utilities|SetState "NewEnumerator5")))
        (else
          (Variables|Default|SetErrorMessage "Session not valid!")
          (Utilities|SetState "NewEnumerator5"))))))

(event Custom|LeaveSession
  (params (OptionalLevel :type Name))
  (|DestroySession (Game|GetPlayerController 0)
    (:OnSuccess
      (Variables|Default|SetCurrentOnlineState "NewEnumerator0")
      (Development|PrintText "Destroyed Session"))
    (:OnFailure
      (Variables|Default|SetErrorMessage "Failed to Destroy current session")
      (Variables|Default|SetCurrentOnlineState "NewEnumerator5")))
  (if (== (Utilities|String|Len (Utilities|String|ToString(Name) OptionalLevel)) 0)
    (Game|OpenLevel(byName) "SNW_entry")
    (else
      (Game|OpenLevel(byName) OptionalLevel))))

(fn SelectBestSession
  (if (> (Utilities|Array|Length (Variables|Default|GetLastSessionSearchResults)) 0)
    (for _array_element (Variables|Default|GetLastSessionSearchResults)
      (if (Class|AdvancedSessionsLibrary|IsValidSession _array_element)
        (return _array_element)))
    (Variables|Default|SetErrorMessage "0 sessions valid!")
    (Utilities|SetState "NewEnumerator7"
      (:SameState
        _)
      (:NewState
        _))
    (return "")
    (else
      (Variables|Default|SetErrorMessage "0 sessions returned!")
      (Utilities|SetState "NewEnumerator7"
        (:SameState
          _)
        (:NewState
          _))
      (return ""))))